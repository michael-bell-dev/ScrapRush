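; BP_Semi is a gun that fires a burst per trigger pull, repeating the selected bullet during the first quarter of its cooldown.
; Shoot snapshots stats and aim, then SelectBullet runs; FireBullet spawns the projectile with those stats and re-triggers via QuadFire.
; QuadFire restores the snapshot so shots match, follows the target or shifts aim with gun movement, then advances to the next bullet when the burst ends.
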(event Custom|TempStore
  ;[1 1 1] Store modifier values every shot so all bullets are the same
  (Variables|Default|SetTempCooldown (Variables|Default|GetCooldown))
  (Variables|Default|SetTempSpeed (Variables|Default|GetBulletVelocity))
  (Variables|Default|SetTempDamage (Variables|Default|GetDamage))
  (Variables|Default|SetTempLifetime (Variables|Default|GetLifetime))
  (Variables|Default|SetTempGravity (Variables|Default|GetGravity))
  (Variables|Default|SetTempHoming (Variables|Default|GetHoming))
  (Variables|Default|SetTempRadius (Variables|Default|GetRadius)))

(event Custom|QuadFire
  (bind _returnvalue (Transformation|GetActorLocation))
  (bind _returnvalue_2 (Transformation|GetActorRotation))
  ;[1 1 1] Loop firing
  (if (Variables|Default|GetKeepFiring)
    (CallFunction|TempReset)
    (Utilities|FlowControl|Delay (/ (Variables|Default|GetCooldownToUse) (Variables|Default|GetSubCooldown)))
    (Variables|Default|SetCurrentBulletIndex (Variables|Default|GetBulletIndexSaved))
    (Utilities|IsValid (Variables|Default|GetTarget)
      (:Is%20Valid
        (Variables|Default|SetHitLocation (+ (Transformation|GetActorLocation (Variables|Default|GetTarget)) "0.000000,0.000000,50.000000")))
      (:Is%20Not%20Valid
        (Variables|Default|SetHitLocation (Math|Vector|RotateVector (Math|Vector|RotateVector (+ (Variables|Default|GetHitLocation) (- (Variables|Default|GetPositionLastBullet) _returnvalue)) (Math|Transform|InverseTransformRotation (Math|Transform|MakeTransform "0, 0, 0" (Variables|Default|GetRotationLastBullet) "1.000000,1.000000,1.000000") "0, 0, 0")) _returnvalue_2))
        (Variables|Default|SetRotationLastBullet _returnvalue_2)
        (Variables|Default|SetPositionLastBullet _returnvalue)))
    (CallFunction|ResetAfterModifiers)
    (CallFunction|SelectBullet)
    (else
      (Utilities|FlowControl|DelayUntilNextTick)
      (CallFunction|NextBullet))))

(event Custom|TempReset
  ;[1 1 1] Store modifier values every shot so all bullets are the same
  (Variables|Default|SetCooldown (Variables|Default|GetTempCooldown))
  (Variables|Default|SetBulletVelocity (Variables|Default|GetTempSpeed))
  (Variables|Default|SetDamage (Variables|Default|GetTempDamage))
  (Variables|Default|SetLifetime (Variables|Default|GetTempLifetime))
  (Variables|Default|SetGravity (Variables|Default|GetTempGravity))
  (Variables|Default|SetHoming (Variables|Default|GetTempHoming))
  (Variables|Default|SetRadius (Variables|Default|GetTempRadius)))

(event EventBeginPlay)

(event Collision|EventActorBeginOverlap
  (params (OtherActor :type Actor%20Object%20Reference)))

(event EventTick
  (params (DeltaSeconds :type Float%20%28single-precision%29)))

(event EventPlayAnimation
  (Components|Animation|PlayAnimation (Variables|Default|GetSkeletalMesh) "/Game/Pickups/MilitaryWeapSilver/Weapons/Animations/Fire_GrenadeLauncher_W.Fire_GrenadeLauncher_W" false))

(event EventCooldownRecovery
  (params (CooldownTime :type Float%20%28double-precision%29))
  (bind _returnvalue (/ CooldownTime 4.0))
  ;[1 1 1] Cooldown between bullets
  (Variables|Default|SetCanShoot false)
  (Utilities|FlowControl|Delay _returnvalue)
  (Variables|Default|SetKeepFiring false)
  ;[1 1 1] Regular cooldown
  (Utilities|FlowControl|Delay (* _returnvalue 3.0))
  (CallFunction|ResetAfterModifiers)
  (Variables|Default|SetCanShoot true))

(fn ConstructionScript
  (|CallParentFunction))

(fn Shoot
  (params (LookingActor :type Scene%20Component%20Object%20Reference) (Target :type Actor%20Object%20Reference))
  (if (Variables|Default|GetCanShoot)
    (CallFunction|TempStore)
    (Variables|Default|SetBulletIndexSaved (Variables|Default|GetCurrentBulletIndex))
    (Variables|Default|SetPositionLastBullet (Transformation|GetActorLocation))
    (Variables|Default|SetRotationLastBullet (Transformation|GetActorRotation))
    (Utilities|IsValid LookingActor
      (:Is%20Valid
        (Variables|Default|SetHitLocation (+ (Transformation|GetWorldLocation LookingActor) (* (Math|Vector|GetForwardVector (Transformation|GetSocketRotation LookingActor "None")) 2e+04))))
      (:Is%20Not%20Valid
        (Variables|Default|SetHitLocation (+ (Transformation|GetActorLocation Target) "0.000000,0.000000,50.000000"))
        (Variables|Default|SetTarget Target)))
    (Variables|Default|SetKeepFiring true)
    (bind _fired (CallFunction|SelectBullet))
    (if _fired
      (CallFunction|PlayAnimation)
      (CallFunction|CooldownRecovery (Variables|Default|GetCooldownToUse))
      (return true)
      (else
        (CallFunction|CooldownRecovery 0.5)
        (return false)))
    (else
      (return false))))

(fn FireBullet
  (params (BulletBP :type Actor%20Class%20Reference))
  (bind _statis (Variables|Default|GetStatis))
  (bind _skeletalmesh (Variables|Default|GetSkeletalMesh))
  (bind _returnvalue (Transformation|GetSocketLocation _skeletalmesh "barrel"))
  (if (== (Variables|Default|GetRandom) 0.0)
    _
    (else
      (CallFunction|RandomHitLocation)))
  (bind _returnvalue_2 (Game|SpawnActorfromClass BulletBP (Math|Transform|MakeTransform _returnvalue "0, 0, 0" "1.000000,1.000000,1.000000") "Undefined" "MultiplyWithRoot" (Components|GetOwner) 0))
  (bind _asbp_projectile_base (Utilities|Casting|CastToBP_ProjectileBase _returnvalue_2))
  (Default|SetStats _asbp_projectile_base (Math|Vector|Normalize (- (Variables|Default|GetHitLocation) _returnvalue) 0.0) (Variables|Default|GetBulletVelocity) (Variables|Default|GetLifetime) (Variables|Default|GetDamage) (Variables|Default|GetPiercing) _statis (Variables|Default|GetInstantActivate) (Variables|Default|GetGravity) (Variables|Default|GetBounce) (Variables|Default|GetPhaseEnemies) (Variables|Default|GetHoming) (Variables|Default|GetRadius) (Variables|Default|GetAttackTarget))
  (if _statis
    (Utilities|Array|Add (Variables|Default|GetBulletsInStatis) _asbp_projectile_base))
  (Variables|Default|SetCooldownToUse (* (Variables|Default|GetCooldown) (Variables|/Game/Pickups/Bullets/BP_ProjectileBase.BP_ProjectileBase_C|GetCooldown _asbp_projectile_base)))
  (CallFunction|QuadFire)
  (return true))