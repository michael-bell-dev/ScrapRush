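; Shotgun weapon Blueprint whose FireBullet spawns three projectiles per shot in a fan.
; One leaves the barrel socket toward HitLocation; two spawn offset along the mesh's forward vector with directions rotated 15 degrees either way around Z.
; Non-zero Random re-rolls the hit location, and each projectile receives the weapon's stats through SetStats.
; The third projectile scales the cooldown, Statis shots are stored in BulletsInStatis, and PlayAnimation plays the fire animation.
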(event EventBeginPlay
  (|CallParentFunction) ; This node is disabled and will not be called.\nDrag off pins to build functionality.
)

(event Collision|EventActorBeginOverlap
  (params (OtherActor :type Actor%20Object%20Reference))
  (|CallParentFunction OtherActor) ; This node is disabled and will not be called.\nDrag off pins to build functionality.
)

(event EventTick
  (params (DeltaSeconds :type Float%20%28single-precision%29))
  (|CallParentFunction DeltaSeconds) ; This node is disabled and will not be called.\nDrag off pins to build functionality.
)

(event EventPlayAnimation
  (Components|Animation|PlayAnimation (Variables|Default|GetSkeletalMesh) "/Game/Pickups/MilitaryWeapSilver/Weapons/Animations/Fire_Shotgun_W.Fire_Shotgun_W" false))

(fn ConstructionScript
  (|CallParentFunction))

(fn FireBullet
  (params (BulletBP :type Actor%20Class%20Reference))
  (bind _returnvalue (Transformation|GetActorLocation))
  (bind _returnvalue_2 (Transformation|GetActorLocation))
  (bind _bulletsinstatis (Variables|Default|GetBulletsInStatis))
  (bind _statis (Variables|Default|GetStatis))
  (bind _skeletalmesh (Variables|Default|GetSkeletalMesh))
  (bind _skeletalmesh_2 (Variables|Default|GetSkeletalMesh))
  (bind _skeletalmesh_3 (Variables|Default|GetSkeletalMesh))
  (bind _returnvalue_3 (Transformation|GetSocketLocation _skeletalmesh_2 "barrel"))
  (bind _returnvalue_4 (Math|Vector|GetForwardVector _skeletalmesh))
  (bind _returnvalue_5 (Transformation|GetSocketLocation _skeletalmesh "barrel"))
  (bind _returnvalue_6 (Transformation|GetSocketLocation _skeletalmesh_3 "barrel"))
  (bind _returnvalue_7 (Math|Vector|GetForwardVector _skeletalmesh_2))
  (bind _returnvalue_8 (* _returnvalue_7 5e+01))
  (bind _returnvalue_9 (* _returnvalue_4 -5e+01))
  (bind _returnvalue_10 (+ _returnvalue_3 _returnvalue_8))
  (bind _returnvalue_11 (+ _returnvalue_5 _returnvalue_9))
  ;[1 1 1] Fire first bullet
  (if (== (Variables|Default|GetRandom) 0.0)
    _
    (else
      (CallFunction|RandomHitLocation)))
  (bind _returnvalue_12 (Game|SpawnActorfromClass BulletBP (Math|Transform|MakeTransform _returnvalue_6 "0, 0, 0" "1.000000,1.000000,1.000000") "Undefined" "MultiplyWithRoot" (Components|GetOwner) 0))
  (bind _asbp_projectile_base (Utilities|Casting|CastToBP_ProjectileBase _returnvalue_12))
  (Default|SetStats _asbp_projectile_base (Math|Vector|Normalize (- (Variables|Default|GetHitLocation) _returnvalue_6) 0.0) (Variables|Default|GetBulletVelocity) (Variables|Default|GetLifetime) (Variables|Default|GetDamage) (Variables|Default|GetPiercing) _statis (Variables|Default|GetInstantActivate) (Variables|Default|GetGravity) (Variables|Default|GetBounce) (Variables|Default|GetPhaseEnemies) (Variables|Default|GetHoming) (Variables|Default|GetRadius) (Variables|Default|GetAttackTarget))
  ;[1 1 1] Fire second bullet
  (if (== (Variables|Default|GetRandom) 0.0)
    _
    (else
      (Variables|Default|SetRandom (+ 1e+01 (Variables|Default|GetRandom)))
      (CallFunction|RandomHitLocation)))
  (bind _returnvalue_13 (Game|SpawnActorfromClass BulletBP (Math|Transform|MakeTransform _returnvalue_11 "0, 0, 0" "1.000000,1.000000,1.000000") "Undefined" "MultiplyWithRoot" (Components|GetOwner) 0))
  (bind _asbp_projectile_base_2 (Utilities|Casting|CastToBP_ProjectileBase _returnvalue_13))
  (Default|SetStats _asbp_projectile_base_2 (Math|Vector|Normalize (- _returnvalue_11 (+ (Math|Vector|RotateVectorAroundAxis (* (Math|Vector|Normalize (- (Variables|Default|GetHitLocation) _returnvalue) 0.0) -2e+04) 15.0 "0.000000,0.000000,1.000000") _returnvalue)) 0.0) (Variables|Default|GetBulletVelocity) (Variables|Default|GetLifetime) (Variables|Default|GetDamage) (Variables|Default|GetPiercing) _statis (Variables|Default|GetInstantActivate) (Variables|Default|GetGravity) (Variables|Default|GetBounce) (Variables|Default|GetPhaseEnemies) (Variables|Default|GetHoming) (Variables|Default|GetRadius) (Variables|Default|GetAttackTarget))
  ;[1 1 1] Fire third bullet
  (if (== (Variables|Default|GetRandom) 0.0)
    _
    (else
      (CallFunction|RandomHitLocation)
      (Variables|Default|SetRandom (+ (Variables|Default|GetRandom) -1e+01))))
  (bind _returnvalue_14 (Game|SpawnActorfromClass BulletBP (Math|Transform|MakeTransform _returnvalue_10 "0, 0, 0" "1.000000,1.000000,1.000000") "Undefined" "MultiplyWithRoot" (Components|GetOwner) 0))
  (bind _asbp_projectile_base_3 (Utilities|Casting|CastToBP_ProjectileBase _returnvalue_14))
  (Default|SetStats _asbp_projectile_base_3 (Math|Vector|Normalize (- _returnvalue_10 (+ (Math|Vector|RotateVectorAroundAxis (* (Math|Vector|Normalize (- (Variables|Default|GetHitLocation) _returnvalue_2) 0.0) -2e+04) -15.0 "0.000000,0.000000,1.000000") _returnvalue_2)) 0.0) (Variables|Default|GetBulletVelocity) (Variables|Default|GetLifetime) (Variables|Default|GetDamage) (Variables|Default|GetPiercing) _statis (Variables|Default|GetInstantActivate) (Variables|Default|GetGravity) (Variables|Default|GetBounce) (Variables|Default|GetPhaseEnemies) (Variables|Default|GetHoming) (Variables|Default|GetRadius) (Variables|Default|GetAttackTarget))
  ;[1 1 1] Weapon cooldown
  (Variables|Default|SetCooldownToUse (* (Variables|Default|GetCooldown) (Variables|/Game/Pickups/Bullets/BP_ProjectileBase.BP_ProjectileBase_C|GetCooldown _asbp_projectile_base_3)))
  ;[1 1 1] Stasis
  (if _statis
    (Utilities|Array|Add _bulletsinstatis _asbp_projectile_base_3)
    (Utilities|Array|Add _bulletsinstatis _asbp_projectile_base_2)
    (Utilities|Array|Add _bulletsinstatis _asbp_projectile_base)
    (return true)
    (else
      (return true))))