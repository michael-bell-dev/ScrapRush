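; BP_Knife is a melee weapon that plugs into a parent weapon's firing flow, with Empty triggering the swing, NextBullet and cooldown recovery.
; A swing runs one sphere overlap trace ahead-right of the knife, dealing doubled, interrupting damage once per BPI_Damagable actor, tracked in DamageArray.
; Each hit also reports a damage event and plays an impact sound.
; A Swing timeline then procedurally animates the knife's relative location and rotation.
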(event EventBeginPlay)

(event Collision|EventActorBeginOverlap
  (params (OtherActor :type Actor%20Object%20Reference)))

(event EventTick
  (params (DeltaSeconds :type Float%20%28single-precision%29)))

(event EventPlayAnimation
  (bind _returnvalue (Transformation|GetActorLocation))
  (bind _returnvalue_2 (Transformation|GetActorForwardVector))
  (bind _returnvalue_3 (Transformation|GetActorRightVector))
  (bind _damage (Variables|Default|GetDamage))
  (bind _rotation (Variables|Default|GetRotation))
  (bind _returnvalue_4 (* _returnvalue_3 5e+01))
  (bind _returnvalue_5 (* _returnvalue_2 2e+01))
  (bind _returnvalue_6 (* _damage 2.0))
  (bind _returnvalue_7 (+ _returnvalue _returnvalue_5))
  (bind _returnvalue_8 (+ _returnvalue_7 _returnvalue_4))
  (Audio|PlaySound2D "/Game/Pickups/MilitaryWeapSilver/Sound/Knife/Cues/KnifeA_Swing_Cue.KnifeA_Swing_Cue" 1.0 1.0 0.0 0 0)
  (bind _outhits (Collision|MultiSphereTraceForObjects _returnvalue_8 _returnvalue_8 75.0 (Utilities|Array|MakeArray "ObjectTypeQuery3" "ObjectTypeQuery6") false (Utilities|Array|MakeArray (Components|GetOwner)) "None"))
  (for _array_element _outhits
    (if (not (Utilities|Array|ContainsItem (Variables|Default|GetDamageArray) 0))
      (bind _asbpi_damagable (Utilities|Casting|CastToBPI_Damagable (.hitactor _array_element)))
      (Default|TakeDamage _asbpi_damagable (Utilities|Struct|MakeS_DamageInfo _returnvalue_6 "NewEnumerator1" "NewEnumerator1" false false false true))
      (Class|AISenseDamage|ReportDamageEvent (.hitactor _array_element) (Components|GetOwner) _returnvalue_6 "0, 0, 0" "0, 0, 0" "None")
      (Utilities|Array|Insert (Variables|Default|GetDamageArray) 0 (Variables|Default|GetDamageArrayIndex))
      (Variables|Default|SetDamageArrayIndex (+ (Variables|Default|GetDamageArrayIndex) 1))
      (Audio|PlaySoundatLocation "/Game/Pickups/MilitaryWeapSilver/Sound/Knife/Cues/Knife_ImpactBody_Cue.Knife_ImpactBody_Cue" (Transformation|GetActorLocation) "0, 0, 0" 1.0 1.0 0.0 0 0 0 0)))
  (Variables|Default|SetDamageArrayIndex 0)
  (Utilities|Array|Clear (Variables|Default|GetDamageArray))
  (bind (_direction _position _rotation_2) (Timeline|Swing PlayFromStart)
    (:Update
      (Transformation|SetActorRelativeLocation (+ (* _position 4e+01) (Variables|Default|GetLocation)))
      (Transformation|SetActorRelativeRotation (Math|Rotator|MakeRotator (+ (* (.x _rotation_2) 4e+01) (.roll _rotation)) (+ (* (.y _rotation_2) 4e+01) (.pitch _rotation)) (+ (* (.z _rotation_2) 4e+01) (.yaw _rotation)))))))

(event EventEmpty
  (CallFunction|PlayAnimation)
  (CallFunction|NextBullet)
  (CallFunction|CooldownRecovery (Variables|Default|GetCooldownToUse)))

(fn ConstructionScript
  (|CallParentFunction))