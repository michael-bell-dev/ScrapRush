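; BP_WeaponPickup is an interactable weapon pickup that carries gun stats, slot count and inventory.
; SetStats stores those values on the actor.
; On Interact, it passes them, the weapon to spawn and itself to BP_Player's SpawnWeaponFunction.
; It destroys itself on success; otherwise it moves just ahead of the player horizontally and matches the player's rotation.
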(event Custom|SetStats
  (params (Cooldown :type Float%20%28double-precision%29) (BulletVelocity :type Float%20%28double-precision%29) (Damage :type Float%20%28double-precision%29) (Lifetime :type Float%20%28double-precision%29) (NumSlots :type Integer) (Inventory :type Array%20of%20E_BulletTypes%20Enums :default "NewEnumerator21"))
  (Variables|Default|SetCooldown Cooldown)
  (Variables|Default|SetBulletVelocity BulletVelocity)
  (Variables|Default|SetDamage Damage)
  (Variables|Default|SetLifetime Lifetime)
  (Variables|Default|SetNumSlots NumSlots)
  (Variables|Default|SetInventory Inventory))

(event EventBeginPlay
  (|CallParentFunction) ; This node is disabled and will not be called.\nDrag off pins to build functionality.
)

(event Collision|EventActorBeginOverlap
  (params (OtherActor :type Actor%20Object%20Reference))
  (|CallParentFunction OtherActor) ; This node is disabled and will not be called.\nDrag off pins to build functionality.
)

(event EventTick
  (params (DeltaSeconds :type Float%20%28single-precision%29))
  (|CallParentFunction DeltaSeconds) ; This node is disabled and will not be called.\nDrag off pins to build functionality.
)

(event EventInteract
  (params (Character%20Picking%20Up :type Actor%20Object%20Reference))
  (bind _asbp_player (Utilities|Casting|CastToBP_Player Character%20Picking%20Up))
  (bind _success (Default|SpawnWeaponFunction _asbp_player (Variables|Default|GetWeaponToSpawn) (Variables|Default|GetCooldown) (Variables|Default|GetBulletVelocity) (Variables|Default|GetDamage) (Variables|Default|GetLifetime) (Variables|Default|GetNumSlots) (Variables|Default|GetInventory) self))
  (if _success
    (Actor|DestroyActor)
    (else
      (Transformation|SetActorLocation (+ (Transformation|GetActorLocation _asbp_player) (* (Transformation|GetActorForwardVector _asbp_player) "50.000000,50.000000,0.000000")) false false)
      (Transformation|SetActorRotation (Transformation|GetActorRotation _asbp_player)))))

(fn ConstructionScript
  (|CallParentFunction))