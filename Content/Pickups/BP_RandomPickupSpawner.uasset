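; Placeholder actor that spawns one of seven random weapon pickups at its location on BeginPlay, then destroys itself.
; It fills the weapon's Inventory with a random slot count, seeding the first slots by chance, with special handling for rocket launcher and knife.
; All branches then share a pass that randomly offsets cooldown, bullet velocity, damage and lifetime.
; A scrap-test block of fixed inventory items is disabled by a constant branch.
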(event EventBeginPlay
  (bind _returnvalue (Transformation|GetActorLocation))
  ;[1 1 1] Select random weapon
  (switch int (Math|Random|RandomInteger 7)
    (:0
      (bind _returnvalue_2 (Game|SpawnActorfromClass "/Game/Pickups/Guns/Pickups/BP_PistolPickup.BP_PistolPickup_C" (Math|Transform|MakeTransform _returnvalue "0, 0, 0" "1.000000,1.000000,1.000000") "Undefined" "MultiplyWithRoot" 0 0))
      ;[1 1 1] Set weapon contents
      (Variables|Default|SetWeaponSpawned _returnvalue_2)
      (if (> (Math|Random|RandomFloat) 0.85) :!label _label
        (Utilities|Array|Insert (Variables|/Game/Pickups/Guns/Pickups/BP_WeaponPickup.BP_WeaponPickup_C|GetInventory (Variables|Default|GetWeaponSpawned)) "NewEnumerator3")
        (else
          (Utilities|Array|Insert (Variables|/Game/Pickups/Guns/Pickups/BP_WeaponPickup.BP_WeaponPickup_C|GetInventory (Variables|Default|GetWeaponSpawned)) "NewEnumerator0")))
      (if (> (Math|Random|RandomFloat) 0.9) :!label _label_2
        (Utilities|Array|Insert (Variables|/Game/Pickups/Guns/Pickups/BP_WeaponPickup.BP_WeaponPickup_C|GetInventory (Variables|Default|GetWeaponSpawned)) "NewEnumerator3" 1)
        (else
          (Utilities|Array|Insert (Variables|/Game/Pickups/Guns/Pickups/BP_WeaponPickup.BP_WeaponPickup_C|GetInventory (Variables|Default|GetWeaponSpawned)) "NewEnumerator21" 1)))
      (bind _output_get (Variables|/Game/Pickups/Guns/Pickups/BP_WeaponPickup.BP_WeaponPickup_C|SetNumSlots (Variables|Default|GetWeaponSpawned) (+ 5 (Math|Random|RandomInteger 10))))
      (for _index (range 2 (- _output_get 1))
        (Utilities|Array|Insert (Variables|/Game/Pickups/Guns/Pickups/BP_WeaponPickup.BP_WeaponPickup_C|GetInventory (Variables|Default|GetWeaponSpawned)) "NewEnumerator21" _index)))
    (:1
      (bind _returnvalue_3 (Game|SpawnActorfromClass "/Game/Pickups/Guns/Pickups/BP_ShotgunPickup.BP_ShotgunPickup_C" (Math|Transform|MakeTransform _returnvalue "0, 0, 0" "1.000000,1.000000,1.000000") "Undefined" "MultiplyWithRoot" 0 0))
      (Variables|Default|SetWeaponSpawned _returnvalue_3)
      (goto _label))
    (:2
      (bind _returnvalue_4 (Game|SpawnActorfromClass "/Game/Pickups/Guns/Pickups/BP_SniperPickup.BP_SniperPickup_C" (Math|Transform|MakeTransform _returnvalue "0, 0, 0" "1.000000,1.000000,1.000000") "Undefined" "MultiplyWithRoot" 0 0))
      (Variables|Default|SetWeaponSpawned _returnvalue_4)
      (goto _label))
    (:3
      (bind _returnvalue_5 (Game|SpawnActorfromClass "/Game/Pickups/Guns/Pickups/BP_SemiPickup.BP_SemiPickup_C" (Math|Transform|MakeTransform _returnvalue "0, 0, 0" "1.000000,1.000000,1.000000") "Undefined" "MultiplyWithRoot" 0 0))
      (Variables|Default|SetWeaponSpawned _returnvalue_5)
      (Variables|/Game/Pickups/Guns/Pickups/BP_SemiPickup.BP_SemiPickup_C|SetSubCooldown _returnvalue_5 (+ (* (Math|Random|RandomFloat) 6.0) 6.0))
      (goto _label))
    (:4
      (bind _returnvalue_6 (Game|SpawnActorfromClass "/Game/Pickups/Guns/Pickups/BP_ARPickup.BP_ARPickup_C" (Math|Transform|MakeTransform _returnvalue "0, 0, 0" "1.000000,1.000000,1.000000") "Undefined" "MultiplyWithRoot" 0 0))
      (Variables|Default|SetWeaponSpawned _returnvalue_6)
      (goto _label))
    (:5
      (bind _returnvalue_7 (Game|SpawnActorfromClass "/Game/Pickups/Guns/Pickups/BP_RocketLauncherPickup.BP_RocketLauncherPickup_C" (Math|Transform|MakeTransform _returnvalue "0, 0, 0" "1.000000,1.000000,1.000000") "Undefined" "MultiplyWithRoot" 0 0))
      (Variables|Default|SetWeaponSpawned _returnvalue_7)
      (Utilities|Array|Insert (Variables|/Game/Pickups/Guns/Pickups/BP_WeaponPickup.BP_WeaponPickup_C|GetInventory (Variables|Default|GetWeaponSpawned)) "NewEnumerator13")
      (goto _label_2))
    (:6
      (bind _returnvalue_8 (Game|SpawnActorfromClass "/Game/Pickups/Guns/Pickups/BP_Knife_Pickup.BP_Knife_Pickup_C" (Math|Transform|MakeTransform _returnvalue "0, 0, 0" "1.000000,1.000000,1.000000") "Undefined" "MultiplyWithRoot" 0 0))
      (Variables|Default|SetWeaponSpawned _returnvalue_8)
      (bind _output_get_2 (Variables|/Game/Pickups/Guns/Pickups/BP_WeaponPickup.BP_WeaponPickup_C|SetNumSlots (Variables|Default|GetWeaponSpawned) (+ 2 (Math|Random|RandomInteger 5))))
      (for _index_2 (range 0 (- _output_get_2 1))
        (Utilities|Array|Insert (Variables|/Game/Pickups/Guns/Pickups/BP_WeaponPickup.BP_WeaponPickup_C|GetInventory (Variables|Default|GetWeaponSpawned)) "NewEnumerator21" _index_2))))
  ;[1 1 1] Set random stats
  (Variables|/Game/Pickups/Guns/Pickups/BP_WeaponPickup.BP_WeaponPickup_C|SetCooldown (Variables|Default|GetWeaponSpawned) (+ (Variables|/Game/Pickups/Guns/Pickups/BP_WeaponPickup.BP_WeaponPickup_C|GetCooldown (Variables|Default|GetWeaponSpawned)) (- (* (Math|Random|RandomFloat) 0.2) 0.07)))
  (Variables|/Game/Pickups/Guns/Pickups/BP_WeaponPickup.BP_WeaponPickup_C|SetBulletVelocity (Variables|Default|GetWeaponSpawned) (+ (Variables|/Game/Pickups/Guns/Pickups/BP_WeaponPickup.BP_WeaponPickup_C|GetBulletVelocity (Variables|Default|GetWeaponSpawned)) (- (* (Math|Random|RandomFloat) 2.0) 1.0)))
  (Variables|/Game/Pickups/Guns/Pickups/BP_WeaponPickup.BP_WeaponPickup_C|SetDamage (Variables|Default|GetWeaponSpawned) (+ (Variables|/Game/Pickups/Guns/Pickups/BP_WeaponPickup.BP_WeaponPickup_C|GetDamage (Variables|Default|GetWeaponSpawned)) (- (Math|Random|RandomFloat) 0.5)))
  (Variables|/Game/Pickups/Guns/Pickups/BP_WeaponPickup.BP_WeaponPickup_C|SetLifetime (Variables|Default|GetWeaponSpawned) (+ (Variables|/Game/Pickups/Guns/Pickups/BP_WeaponPickup.BP_WeaponPickup_C|GetLifetime (Variables|Default|GetWeaponSpawned)) (- (* (Math|Random|RandomFloat) 0.2) 0.1)))
  ;[1 1 1] SCRAP TEST
  (if true
    (Actor|DestroyActor)
    (else
      (Utilities|Array|SetArrayElem (Variables|/Game/Pickups/Guns/Pickups/BP_WeaponPickup.BP_WeaponPickup_C|GetInventory (Variables|Default|GetWeaponSpawned)) 0 "NewEnumerator18")
      (Utilities|Array|SetArrayElem (Variables|/Game/Pickups/Guns/Pickups/BP_WeaponPickup.BP_WeaponPickup_C|GetInventory (Variables|Default|GetWeaponSpawned)) 1 "NewEnumerator18")
      (Utilities|Array|SetArrayElem (Variables|/Game/Pickups/Guns/Pickups/BP_WeaponPickup.BP_WeaponPickup_C|GetInventory (Variables|Default|GetWeaponSpawned)) 2 "NewEnumerator18")
      (Utilities|Array|SetArrayElem (Variables|/Game/Pickups/Guns/Pickups/BP_WeaponPickup.BP_WeaponPickup_C|GetInventory (Variables|Default|GetWeaponSpawned)) 3 "NewEnumerator18")
      (Utilities|Array|SetArrayElem (Variables|/Game/Pickups/Guns/Pickups/BP_WeaponPickup.BP_WeaponPickup_C|GetInventory (Variables|Default|GetWeaponSpawned)) 4 "NewEnumerator12")
      (Actor|DestroyActor))))

(fn ConstructionScript)