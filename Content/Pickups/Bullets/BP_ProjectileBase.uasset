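; Base projectile for weapon bullets, configured by SetStats, with optional gravity, bounce, piercing, homing, instant activation and stasis.
; Slow or bouncing shots use projectile movement and overlaps, while fast ones switch to line traces, aimed from the camera for players.
; Homing follows AttackTarget or sphere-traces for nearby pawns, and stasis holds shots until UnStatis relaunches them.
; Hits feed CollisionBehavior, which damages BPI_Damagable actors and destroys non-piercing projectiles, while BP_Bubble intercepts traced shots.
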(event OnComponentBeginOverlap(Sphere)
  (params (OverlappedComponent :type Primitive%20Component%20Object%20Reference) (OtherActor :type Actor%20Object%20Reference) (OtherComp :type Primitive%20Component%20Object%20Reference) (OtherBodyIndex :type Integer) (bFromSweep :type Boolean) (SweepResult :type Hit%20Result%20Structure%20%28by%20ref%29))
  ;[1 1 1] Collision function
  (if (Variables|Default|GetValuesUpdated)
    _
    (else
      (Utilities|FlowControl|DelayUntilNextTick)))
  (if (not (Variables|Default|GetStatis))
    (Utilities|Casting|CastToBP_ProjectileBase OtherActor
      (:CastFailed
        (if (Variables|Default|GetPhaseEnemies)
          (Utilities|Casting|CastToBPI_Damagable OtherActor
            (:CastFailed
              _)))
        (CallFunction|CollisionBehavior (Transformation|GetActorLocation) OtherActor)))))

(event Custom|KillEventually
  ;[1 1 1] Destroy after certain amount of time
  (Utilities|FlowControl|Delay (Variables|Default|GetLifetime))
  (if (not (Variables|Default|GetCancelDeletion))
    (Actor|DestroyActor)))

(event Custom|CollisionBehavior
  (params (Location :type Vector) (DamagedActor :type Actor%20Object%20Reference))
  ;[1 1 1] Unique bullet behavior
  (Utilities|Casting|CastToBPI_Damagable DamagedActor
    (:then
      (Class|BPIDamagable|TakeDamage(Message) DamagedActor (Utilities|Struct|MakeS_DamageInfo (Variables|Default|GetDamage) "NewEnumerator2" "NewEnumerator1" false false false true))
      (Class|AISenseDamage|ReportDamageEvent DamagedActor (Components|GetOwner) (Variables|Default|GetDamage) "0, 0, 0" "0, 0, 0" "None"))
    (:CastFailed
      _))
  (if (not (>= (Variables|Default|GetPiercing) 1))
    (Actor|DestroyActor)))

(event Custom|DoLineTrace
  (bind _returnvalue (Components|GetOwner))
  (bind _array (Utilities|Array|MakeArray "ObjectTypeQuery1" "ObjectTypeQuery2" "ObjectTypeQuery3" "ObjectTypeQuery4" "ObjectTypeQuery6"))
  (bind _array_2 (Utilities|Array|MakeArray _returnvalue))
  ;[1 1 1] Use line trace if velocity is high
  (bind _asbp_player (Utilities|Casting|CastToBP_Player (Components|GetOwner))
    (:then
      (bind _output_get (Variables|Default|SetStartPos (Transformation|GetWorldLocation (Variables|/Game/Characters/Player/BP_Player.BP_Player_C|GetFollowCamera _asbp_player))))
      (Variables|Default|SetDirection (+ _output_get (* (Math|Vector|GetForwardVector (Variables|/Game/Characters/Player/BP_Player.BP_Player_C|GetFollowCamera _asbp_player)) 2e+04 (Variables|Default|GetLifetime)))))
    (:CastFailed
      (Variables|Default|SetDirection (* (Variables|Default|GetDirection) 2e+04))))
  (Utilities|FlowControl|DelayUntilNextTick)
  (if (>= (Variables|Default|GetPiercing) 1)
    (bind _outhits (Class|KismetSystemLibrary|LineTraceMultiforObjects (Variables|Default|GetStartPos) (Variables|Default|GetDirection) _array false _array_2 "None" true))
    (bind _array_element (Utilities|Array|ForEachLoopwithBreak _outhits :!label _label)
      (:LoopBody
        (switch Utilities|FlowControl|Switch|SwitchonEComponentMobility (Variables|/Script/Engine.SceneComponent|GetMobility (.hitcomponent _array_element))
          (:Static
            (if (> (Variables|Default|GetPiercing) 1)
              _
              (else
                (goto _label Break))))
          (:Stationary
            _)
          (:Movable
            _))
        (bind _asbp_bubble (Utilities|Casting|CastToBP_Bubble (.hitactor _array_element))
          (:then
            (Default|AbsorborCollide _asbp_bubble self)
            (goto _label Break))
          (:CastFailed
            (if (not (Utilities|Array|ContainsItem (Variables|Default|GetHitArray) 0))
              (Utilities|Array|Add (Variables|Default|GetHitArray) 0)
              (CallFunction|CollisionBehavior "0, 0, 0")))))
      (:Completed
        (CallFunction|KillEventually)))
    (else
      (bind (_outhit _returnvalue_2) (Collision|LineTraceForObjects (Variables|Default|GetStartPos) (Variables|Default|GetDirection) _array false _array_2 "None"))
      (if _returnvalue_2
        (bind _asbp_bubble_2 (Utilities|Casting|CastToBP_Bubble (.hitactor _outhit))
          (:then
            (Default|AbsorborCollide _asbp_bubble_2 self))
          (:CastFailed
            (CallFunction|CollisionBehavior (.impactpoint _outhit) (.hitactor _outhit))))))))

(event Custom|SetStats
  (params (Direction :type Vector) (Velocity :type Float%20%28double-precision%29) (Lifetime :type Float%20%28double-precision%29) (Damage :type Float%20%28double-precision%29) (Piercing :type Integer) (Statis :type Boolean) (InstantActivate :type Boolean) (Gravity :type Float%20%28double-precision%29) (Bounce :type Boolean) (PhaseEnemies :type Boolean) (Homing :type Float%20%28double-precision%29) (Radius :type Float%20%28double-precision%29) (AttackTarget :type Actor%20Object%20Reference))
  ;[1 1 1] Set values according to weapon
  (bind _output_get (Variables|Default|SetDirection (* Direction (* Velocity (Variables|Default|GetVelocity)))))
  (bind _output_get_2 (Variables|/Script/Engine.MovementComponent|SetVelocity (Variables|Default|GetProjectileMovement) _output_get))
  (Variables|Default|SetDoPhysicsCalculation (< (Math|Vector|VectorLength _output_get_2) 5e+03))
  (Variables|Default|SetLifetime (* (Variables|Default|GetLifetime) Lifetime))
  (Variables|Default|SetDamage (* (Variables|Default|GetDamage) Damage))
  (Variables|Default|SetPiercing (+ (Variables|Default|GetPiercing) Piercing))
  (Variables|Default|SetStatis Statis)
  (Variables|Default|SetInstantActivate (or InstantActivate (Variables|Default|GetInstantActivate)))
  (Variables|Default|SetGravity (+ (Variables|Default|GetGravity) Gravity))
  (Variables|Default|SetBounce (or Bounce (Variables|Default|GetBounce)))
  (Variables|Default|SetPhaseEnemies (or PhaseEnemies (Variables|Default|GetPhaseEnemies)))
  (Variables|Default|SetHoming (+ (Variables|Default|GetHoming) Homing))
  (Variables|Default|SetRadius (* (Variables|Default|GetRadius) Radius))
  (Variables|Default|SetAttackTarget AttackTarget))

(event EventBeginPlay
  (bind _returnvalue (Transformation|GetActorForwardVector))
  (bind _returnvalue_2 (Components|GetOwner))
  (bind _returnvalue_3 (Transformation|GetActorLocation))
  (bind _sphere (Variables|Default|GetSphere))
  (bind _attacktarget (Variables|Default|GetAttackTarget))
  (bind _returnvalue_4 (* _returnvalue 1e+03))
  (bind _returnvalue_5 (+ _returnvalue_3 _returnvalue_4))
  ;[1 1 1] Initialization
  (Variables|Default|SetStartPos (Transformation|GetActorLocation))
  (Utilities|FlowControl|DelayUntilNextTick)
  (Variables|Default|SetValuesUpdated true)
  (if (> (Variables|Default|GetPiercing) 1)
    (Collision|SetCollisionResponsetoChannel (Variables|Default|GetSphere1) "ECC_WorldStatic" "ECR_Ignore"))
  (if (Variables|Default|GetStatis)
    (Game|Components|ProjectileMovement|SetVelocityinLocalSpace (Variables|Default|GetProjectileMovement) "0, 0, 0")
    (else
      (if (Variables|Default|GetInstantActivate)
        (CallFunction|CollisionBehavior (Transformation|GetActorLocation _returnvalue_2) _returnvalue_2)
        (Utilities|IsValid self
          (:Is%20Valid
            _)))
      ;[1 1 1] Homing
      (Variables|/Script/Engine.ProjectileMovementComponent|SetProjectileGravityScale (Variables|Default|GetProjectileMovement) (Variables|Default|GetGravity))
      (if (!= (Variables|Default|GetHoming) 0.0)
        (Variables|/Script/Engine.ProjectileMovementComponent|SetbIsHomingProjectile (Variables|Default|GetProjectileMovement) true)
        (Utilities|IsValid _attacktarget
          (:Is%20Valid
            (Variables|/Script/Engine.ProjectileMovementComponent|SetHomingTargetComponent (Variables|Default|GetProjectileMovement) (Variables|/Game/Characters/Player/BP_Player.BP_Player_C|GetCapsule (.AsBP%20Player (Utilities|Casting|CastToBP_Player _attacktarget)))))
          (:Is%20Not%20Valid
            (bind _outhits (Collision|MultiSphereTraceForObjects _returnvalue_5 _returnvalue_5 1.5e+03 (Utilities|Array|MakeArray "ObjectTypeQuery3") false (Utilities|Array|MakeArray (Components|GetOwner)) "None"))
            (for _array_element _outhits
              (Utilities|Array|Insert (Variables|Default|GetHomingArray) (.hitactor _array_element))
              (bind _asbp_enemy_base (Utilities|Casting|CastToBP_Enemy_Base (.hitactor _array_element))
                (:then
                  (bind _isdead (Default|IsDead _asbp_enemy_base))
                  (if (not _isdead)
                    (if (< (Transformation|GetDistanceTo (.hitactor _array_element) self) (Variables|Default|GetMinDistance)) :!label _label
                      (Variables|Default|SetMinDistance (Transformation|GetDistanceTo (.hitactor _array_element) self))
                      (Variables|/Script/Engine.ProjectileMovementComponent|SetHomingTargetComponent (Variables|Default|GetProjectileMovement) (Variables|/Script/Engine.Actor|GetRootComponent (.hitactor _array_element))))))
                (:CastFailed
                  (goto _label))))))
        (Variables|/Script/Engine.ProjectileMovementComponent|SetHomingAccelerationMagnitude (Variables|Default|GetProjectileMovement) (Variables|Default|GetHoming)))
      ;[1 1 1] Bounce
      (if (Variables|Default|GetBounce)
        (Variables|/Script/Engine.ProjectileMovementComponent|SetbShouldBounce (Variables|Default|GetProjectileMovement) true)
        (Collision|SetCollisionResponsetoChannel _sphere "ECC_WorldStatic" "ECR_Block")
        (Collision|SetCollisionResponsetoChannel _sphere "ECC_PhysicsBody" "ECR_Block")
        (Variables|/Script/Engine.PrimitiveComponent|SetbGenerateOverlapEvents (Variables|Default|GetSphere) true :!label _label_2)
        (CallFunction|KillEventually)
        (elif (Variables|Default|GetDoPhysicsCalculation)
          (goto _label_2)
          (else
            (CallFunction|DoLineTrace)))))))

(fn ConstructionScript)

(fn UnStatis
  (bind _returnvalue (Transformation|GetActorForwardVector))
  (bind _returnvalue_2 (Transformation|GetActorLocation))
  (bind _sphere (Variables|Default|GetSphere))
  (bind _attacktarget (Variables|Default|GetAttackTarget))
  (bind _returnvalue_3 (* _returnvalue 1e+03))
  (bind _returnvalue_4 (+ _returnvalue_2 _returnvalue_3))
  (Variables|/Script/Engine.MovementComponent|SetVelocity (Variables|Default|GetProjectileMovement) (Variables|Default|GetDirection))
  (Variables|Default|SetStatis false)
  (if (Variables|Default|GetInstantActivate)
    (CallFunction|CollisionBehavior (Transformation|GetActorLocation) (Utilities|Array|Get(acopy) (Collision|GetOverlappingActors (Variables|Default|GetSphere) "/Game/Characters/Enemies/BP_Enemy_Base.BP_Enemy_Base_C" :!class /Script/Engine.PrimitiveComponent)))
    (Utilities|IsValid self
      (:Is%20Valid
        _)))
  (Variables|/Script/Engine.ProjectileMovementComponent|SetProjectileGravityScale (Variables|Default|GetProjectileMovement) (Variables|Default|GetGravity))
  (if (!= (Variables|Default|GetHoming) 0.0)
    (Variables|/Script/Engine.ProjectileMovementComponent|SetbIsHomingProjectile (Variables|Default|GetProjectileMovement) true)
    (Utilities|IsValid _attacktarget
      (:Is%20Valid
        (Variables|/Script/Engine.ProjectileMovementComponent|SetHomingTargetComponent (Variables|Default|GetProjectileMovement) (Variables|/Game/Characters/Player/BP_Player.BP_Player_C|GetCapsule (.AsBP%20Player (Utilities|Casting|CastToBP_Player _attacktarget))))
        (Variables|/Script/Engine.ProjectileMovementComponent|SetHomingAccelerationMagnitude (Variables|Default|GetProjectileMovement) (Variables|Default|GetHoming)))
      (:Is%20Not%20Valid
        (bind _outhits (Collision|MultiSphereTraceForObjects _returnvalue_4 _returnvalue_4 1.5e+03 (Utilities|Array|MakeArray "ObjectTypeQuery3") false (Utilities|Array|MakeArray (Components|GetOwner)) "None"))
        (for _array_element _outhits
          (Utilities|Array|Insert (Variables|Default|GetHomingArray) (.hitactor _array_element))
          (bind _asbp_enemy_base (Utilities|Casting|CastToBP_Enemy_Base (.hitactor _array_element))
            (:then
              (bind _isdead (Default|IsDead _asbp_enemy_base))
              (if (not _isdead)
                (if (< (Transformation|GetDistanceTo (.hitactor _array_element) self) (Variables|Default|GetMinDistance)) :!label _label
                  (Variables|Default|SetMinDistance (Transformation|GetDistanceTo (.hitactor _array_element) self))
                  (Variables|/Script/Engine.ProjectileMovementComponent|SetHomingTargetComponent (Variables|Default|GetProjectileMovement) (Variables|/Script/Engine.Actor|GetRootComponent (.hitactor _array_element))))))
            (:CastFailed
              (goto _label)))))))
  (if (Variables|Default|GetBounce)
    (Variables|/Script/Engine.ProjectileMovementComponent|SetbShouldBounce (Variables|Default|GetProjectileMovement) true)
    (Collision|SetCollisionResponsetoChannel _sphere "ECC_WorldStatic" "ECR_Block")
    (Collision|SetCollisionResponsetoChannel _sphere "ECC_Destructible" "ECR_Block")
    (Variables|/Script/Engine.PrimitiveComponent|SetbGenerateOverlapEvents (Variables|Default|GetSphere) true :!label _label_2)
    (CallFunction|KillEventually)
    (elif (Variables|Default|GetDoPhysicsCalculation)
      (goto _label_2)
      (else
        (CallFunction|DoLineTrace)))))