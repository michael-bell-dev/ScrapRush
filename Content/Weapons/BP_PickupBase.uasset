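; Base pickup Blueprint that registers itself with the player's cullable actor list on spawn and leaves Interact empty.
; AddPriceTag turns it into a shop item, deriving a price from its value, a random discount and the player's room number, with a minimum floor.
; The price shows in a W_Price widget, which is hidden unless a ShopReader overlaps the pickup's sphere.
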(event Custom|Add%20Price%20Tag
  (Variables|Default|SetShopItem true)
  (Variables|Default|SetValue (Math|Integer|Max(Integer) (* (+ (Variables|Default|GetValue) (* (Math|Random|RandomInteger 50) -1) (Variables|/Game/Characters/Player/BP_Player.BP_Player_C|GetRoomNum (.AsBP%20Player (Utilities|Casting|CastToBP_Player (Game|Player|GetPlayerPawn 0))))) 5) 10))
  (bind _returnvalue (UserInterface|CreateWidget "/Game/Weapons/W_Price.W_Price_C"))
  (UserInterface|SetWidget (Variables|Default|GetWidget) _returnvalue)
  (Default|SetPrice _returnvalue (Variables|Default|GetValue))
  (if (== (Utilities|Array|Length (Collision|GetOverlappingActors (Variables|Default|GetSphere) "/Game/Characters/Player/ShopReader.ShopReader_C" :!class /Script/Engine.PrimitiveComponent)) 0)
    (Rendering|SetVisibility (Variables|Default|GetWidget) false true)))

(event EventBeginPlay
  (bind _asbp_player (Utilities|Casting|CastToBP_Player (Game|Player|GetPlayerPawn 0)))
  (Utilities|Array|Add (Variables|/Game/Characters/Player/BP_Player.BP_Player_C|GetCullableActors _asbp_player) self))

(event EventInteract
  (params (Character%20Picking%20Up :type Actor%20Object%20Reference)))

(fn ConstructionScript)