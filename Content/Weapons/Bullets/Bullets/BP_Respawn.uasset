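; BP_Respawn is a bullet Blueprint that resets room content state when its collision behavior fires.
; CollisionBehavior finds every Master_Room actor and clears its ContentGenerated flag, then passes the damaged actor to EndOfLife.
; It does not regenerate rooms itself, as the GenerateContent call is left unconnected.
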(event Collision|EventActorBeginOverlap
  (params (OtherActor :type Actor%20Object%20Reference))
  (|CallParentFunction OtherActor) ; This node is disabled and will not be called.\nDrag off pins to build functionality.
)

(event EventTick
  (params (DeltaSeconds :type Float%20%28single-precision%29))
  (|CallParentFunction DeltaSeconds) ; This node is disabled and will not be called.\nDrag off pins to build functionality.
)

(event EventCollisionBehavior
  (params (Location :type Vector :default "0, 0, 0") (DamagedActor :type Actor%20Object%20Reference) (HitComponent :type Primitive%20Component%20Object%20Reference))
  (bind _outactors (Actor|GetAllActorsOfClass "/Game/Rooms/Rooms/Master_Room.Master_Room_C"))
  (for _array_element _outactors
    (Variables|/Game/Rooms/Rooms/Master_Room.Master_Room_C|SetContentGenerated _array_element false))
  (CallFunction|EndOfLife DamagedActor))

(fn ConstructionScript
  (|CallParentFunction))