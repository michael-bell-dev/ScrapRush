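; Lightning bullet that zaps the actor it hits, then chains damage to nearby living damageable pawns.
; Each jump sphere-traces around the last strike point, skips targets already in DamageArray, deals blockable damage, and draws a short-lived spline arc with Niagara zap effects.
; Lifetime scales the jump limit, and the chain ends early when targets run out.
; EndOfLife runs afterward, or immediately if the hit actor is not damageable.
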(event EventCollisionBehavior
  (params (Location :type Vector :default "0, 0, 0") (DamagedActor :type Actor%20Object%20Reference) (HitComponent :type Primitive%20Component%20Object%20Reference))
  (bind _damage_array (Variables|Default|GetDamage%20Array))
  (bind _output_get (Variables|Default|SetCurPoint Location))
  (Niagara|SpawnSystematLocation "/Game/Vefects/Zap_VFX/VFX/Zap/Particles/NS_Zap_02_Blue.NS_Zap_02_Blue" _output_get)
  (Utilities|Array|Add (Variables|Default|GetDamage%20Array) (Components|GetOwner))
  (Utilities|Casting|CastToBPI_Damagable DamagedActor
    (:then
      (CallFunction|DealDamage DamagedActor true)
      (Utilities|Array|Add (Variables|Default|GetDamage%20Array) DamagedActor)
      (bind _index (Utilities|FlowControl|ForLoopwithBreak 0 (Math|Float|Truncate (* (+ (Variables|Default|GetLifetime) 1.0) 3.0)) :!label _label)
        (:LoopBody
          (if (Utilities|Array|IsValidIndex (Variables|Default|GetDamage%20Array) _index)
            (Variables|Default|SetPrevPoint (Variables|Default|GetCurPoint))
            (bind _outhits (Collision|MultiSphereTraceForObjects (Variables|Default|GetCurPoint) (Variables|Default|GetCurPoint) (Variables|Default|GetRadius) (Utilities|Array|MakeArray "ObjectTypeQuery3") false (Utilities|Array|MakeArray (Components|GetOwner)) "None"))
            (bind _array_element (Utilities|Array|ForEachLoopwithBreak _outhits :!label _label_2)
              (:LoopBody
                (Utilities|Casting|CastToBPI_Damagable (.HitActor (Collision|BreakHitResult _array_element)))
                (if (not (Utilities|Array|ContainsItem (Variables|Default|GetDamage%20Array) (.HitActor (Collision|BreakHitResult _array_element))))
                  (bind _isdead (Class|BPIDamagable|IsDead(Message) (.HitActor (Collision|BreakHitResult _array_element))))
                  (if (not _isdead)
                    (bind _returnvalue (Utilities|Array|Add _damage_array (.HitActor (Collision|BreakHitResult _array_element))))
                    (bind _output_get_2 (Variables|Default|SetCurPoint (Transformation|GetActorLocation (Utilities|Array|Get(acopy) _damage_array _returnvalue))))
                    (bind _returnvalue_2 (Game|SpawnActorfromClass "/Game/Weapons/Bullets/Bullets/SplineObject.SplineObject_C" (Math|Transform|MakeTransform "0, 0, 0" "0, 0, 0" "1.000000,1.000000,1.000000") "Undefined" "MultiplyWithRoot" 0 0))
                    (Default|SetPoints _returnvalue_2 (Variables|Default|GetPrevPoint) _output_get_2 0.1)
                    (Niagara|SpawnSystematLocation "/Game/Vefects/Zap_VFX/VFX/Zap/Particles/NS_Zap_02_Blue.NS_Zap_02_Blue" _output_get_2 (Math|Rotator|FindLookatRotation (Variables|Default|GetPrevPoint) _output_get_2))
                    (CallFunction|DealDamage (.HitActor (Collision|BreakHitResult _array_element)) true)
                    (goto _label_2 Break)))))
            (else
              (goto _label Break))))
        (:Completed
          (CallFunction|EndOfLife DamagedActor :!label _label_3))))
    (:CastFailed
      (goto _label_3))))

(fn ConstructionScript
  (|CallParentFunction))