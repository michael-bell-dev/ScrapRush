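; BP_Sawblade is a sawblade projectile that extends a parent bullet and spins its mesh around yaw every tick.
; In bullet-field mode with a nonzero Offset, it teleports its collider to that offset from its owner, falling back to the player pawn.
; Tick also has spiral and acceleration branches, but their time inputs are zero, so the spiral phase never advances and velocity scaling has no effect.
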(event EventTick
  (params (DeltaSeconds :type Float%20%28single-precision%29))
  (bind _returnvalue (Components|GetOwner))
  (bind _collider (Variables|Default|GetCollider))
  (bind _offset (Variables|Default|GetOffset))
  (bind _projectilemovement (Variables|Default|GetProjectileMovement))
  (bind _acceleration (Variables|Default|GetAcceleration))
  (bind _spiral (Variables|Default|GetSpiral))
  (Transformation|AddLocalRotation (Variables|Default|GetBullet) (Math|Rotator|MakeRotator 0.0 0.0 (* DeltaSeconds 4e+02)) false false)
  (if (and (Variables|Default|GetBulletField) (Utilities|Operators|NotEqual(!=) :A _offset))
    (Utilities|IsValid _returnvalue
      (:Is%20Valid
        (Transformation|SetWorldLocation _collider (+ (Transformation|GetActorLocation _returnvalue) _offset) false true))
      (:Is%20Not%20Valid
        (Transformation|SetWorldLocation _collider (+ _offset (Transformation|GetActorLocation (Game|Player|GetPlayerPawn 0))) false true))))
  (if (== (Variables|Default|GetSpiral) 0.0)
    _
    (else
      (Variables|Default|SetTotalSeconds (+ (Variables|Default|GetTotalSeconds) 0.0))
      (Transformation|AddRelativeLocation (Variables|Default|GetCollider) (Math|Vector|MakeVector 0.0 (* (Math|Trig|Cos(Radians) (* (+ (Variables|Default|GetTotalSeconds) 0.0) (/ (Variables|Default|GetVelocity) 2e+02))) _spiral) (* (Math|Trig|Sin(Radians) (* (+ (Variables|Default|GetTotalSeconds) 0.0) (/ (Variables|Default|GetVelocity) 2e+02))) _spiral)) false false)))
  (if (not (== _acceleration 1.0))
    (Variables|/Script/Engine.MovementComponent|SetVelocity _projectilemovement (* (Variables|/Script/Engine.MovementComponent|GetVelocity _projectilemovement) (Math|Float|Power _acceleration (* 0.0 6e+01))))))

(event EventDestroyed
  (Actor|Tick|SetActorTickEnabled false))

(event EventBeginPlay
  (|CallParentFunction)
  (Actor|Tick|SetActorTickEnabled true))

(fn ConstructionScript
  (|CallParentFunction))