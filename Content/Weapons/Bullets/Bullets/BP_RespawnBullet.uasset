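; BP_RespawnBullet is a bullet that regenerates the content of the room the player is in when it hits.
; Its CollisionBehavior event finds every Master_Room overlapping the player 0 capsule, clears ContentGenerated and calls GenerateContent on each.
; It then passes the damaged actor to EndOfLife; the rooms are chosen by player position, independent of what was hit.
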(event Collision|EventActorBeginOverlap
  (params (OtherActor :type Actor%20Object%20Reference))
  (|CallParentFunction OtherActor) ; This node is disabled and will not be called.\nDrag off pins to build functionality.
)

(event EventTick
  (params (DeltaSeconds :type Float%20%28single-precision%29))
  (|CallParentFunction DeltaSeconds) ; This node is disabled and will not be called.\nDrag off pins to build functionality.
)

(event EventCollisionBehavior
  (params (Location :type Vector :default "0, 0, 0") (DamagedActor :type Actor%20Object%20Reference) (HitComponent :type Primitive%20Component%20Object%20Reference))
  (for _array_element (Collision|GetOverlappingActors (Variables|/Script/Engine.Character|GetCapsuleComponent (.AsBP%20Player (Utilities|Casting|CastToBP_Player (Game|Player|GetPlayerPawn 0)))) "/Game/Rooms/Rooms/Master_Room.Master_Room_C" :!class /Script/Engine.PrimitiveComponent)
    (Variables|/Game/Rooms/Rooms/Master_Room.Master_Room_C|SetContentGenerated (.AsMaster%20Room (Utilities|Casting|CastToMaster_Room _array_element)) false)
    (Default|GenerateContent (.AsMaster%20Room (Utilities|Casting|CastToMaster_Room _array_element))))
  (CallFunction|EndOfLife DamagedActor))

(fn ConstructionScript
  (|CallParentFunction))