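; BP_Aura is a bullet Blueprint that turns a hit into an area burst around the damaged actor.
; Its CollisionBehavior event gathers nearby pawns with a short vertical sphere trace, excludes the hit actor, and deals blockable damage to the rest.
; A radial impulse then fires at the hit location, with strength scaled by Damage and size by Radius.
; It finally calls Yellow on damagable targets and runs EndOfLife.
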(event EventBeginPlay
  (|CallParentFunction) ; This node is disabled and will not be called.\nDrag off pins to build functionality.
)

(event Collision|EventActorBeginOverlap
  (params (OtherActor :type Actor%20Object%20Reference)))

(event EventTick
  (params (DeltaSeconds :type Float%20%28single-precision%29)))

(event EventCollisionBehavior
  (params (Location :type Vector :default "0, 0, 0") (DamagedActor :type Actor%20Object%20Reference) (HitComponent :type Primitive%20Component%20Object%20Reference))
  (bind _returnvalue (Transformation|GetActorLocation DamagedActor))
  (bind _radialforce (Variables|Default|GetRadialForce))
  (bind _overlapping_actors (Variables|Default|GetOverlapping%20Actors))
  (Variables|/Script/Engine.RadialForceComponent|SetForceStrength (Variables|Default|GetRadialForce) (* (Variables|Default|GetDamage) 4e+03))
  (bind _outhits (Collision|MultiSphereTraceForObjects (- _returnvalue "0.000000,0.000000,30.000000") (- _returnvalue "0.000000,0.000000,-30.000000") (/ (Variables|Default|GetRadius) 5.5) (Utilities|Array|MakeArray "ObjectTypeQuery3") false 0 "None"))
  (for _array_element _outhits
    (Utilities|Set|Add (Variables|Default|GetOverlapping%20Actors) (.hitactor _array_element)))
  (Utilities|Set|Remove _overlapping_actors DamagedActor)
  (bind _result (Utilities|Set|ToArray _overlapping_actors))
  (for _array_element_2 _result
    (CallFunction|DealDamage _array_element_2 true))
  (Transformation|SetWorldLocation _radialforce _returnvalue false false)
  (Variables|/Script/Engine.RadialForceComponent|SetRadius _radialforce (/ (Variables|Default|GetRadius) 2.0))
  (Class|RadialForceComponent|FireImpulse (Variables|Default|GetRadialForce))
  (bind _asbpi_damagable (Utilities|Casting|CastToBPI_Damagable DamagedActor)
    (:then
      (Default|Yellow _asbpi_damagable))
    (:CastFailed
      _))
  (CallFunction|EndOfLife DamagedActor))

(fn ConstructionScript
  (|CallParentFunction))