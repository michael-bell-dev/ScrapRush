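; BP_Explosive is an explosive bullet that detonates through CollisionBehavior, with particles scaled by Radius, a sound, a noise event and damage.
; KillEventually detonates it at the collider's location after Lifetime and destroys it, unless CancelDeletion is set.
; Damage is delegated to TEMPORARYAttackInRange before EndOfLife runs.
; An older sphere-trace damage chain, hitting each actor once via DamageArray, remains disconnected.
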(event EventCollisionBehavior
  (params (Location :type Vector :default "0, 0, 0") (DamagedActor :type Actor%20Object%20Reference) (HitComponent :type Primitive%20Component%20Object%20Reference))
  (Effects|SpawnEmitteratLocation "/Game/M5VFXVOL2/Particles/Explosion/Fire_Exp_00.Fire_Exp_00" Location "0, 0, 0" (Math|Conversions|ToVector(Float) (/ (Variables|Default|GetRadius) 3e+02)) true "AutoRelease")
  (Audio|PlaySoundatLocation "/Game/StarterContent/Audio/Explosion_Cue.Explosion_Cue" Location "0, 0, 0" 1.0 1.0 0.0 0 0 0 0)
  (Class|Actor|MakeNoise 1.0 0 Location 0.0 "None")
  (CallFunction|TEMPORARYAttackinRange)
  (CallFunction|EndOfLife))

(event EventKillEventually
  (Utilities|FlowControl|Delay (Variables|Default|GetLifetime))
  (if (not (Variables|Default|GetCancelDeletion))
    (CallFunction|CollisionBehavior (Transformation|GetWorldLocation (Variables|Default|GetCollider)))
    (Actor|DestroyActor)))

(fn ConstructionScript
  (|CallParentFunction))