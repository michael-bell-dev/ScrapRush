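; Black hole bullet that stops in place and damages every BP_Enemy_Base in the level, regardless of distance.
; CollisionBehavior, called on BeginPlay unless Stasis is set, zeroes velocity and grows a sphere through a timeline.
; When that finishes, it deals fixed heavy damage, reports the Damage variable per enemy, then scales a second sphere.
; A lifetime timer can also re-trigger the collapse before destroying the actor.
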(event OnComponentBeginOverlap(Collider)
  (params (OverlappedComponent :type Primitive%20Component%20Object%20Reference) (OtherActor :type Actor%20Object%20Reference) (OtherComp :type Primitive%20Component%20Object%20Reference) (OtherBodyIndex :type Integer) (bFromSweep :type Boolean) (SweepResult :type Hit%20Result%20Structure%20%28by%20ref%29)))

(event EventBeginPlay
  (|CallParentFunction)
  (if (not (Variables|Default|GetStasis))
    (CallFunction|CollisionBehavior "0, 0, 0")))

(event EventDoKill
  (CallFunction|CollisionBehavior "0, 0, 0")
  (Utilities|FlowControl|Delay 2.7)
  (Actor|DestroyActor))

(event EventKillEventually
  (Utilities|Time|SetTimerbyEvent (delegate EventDoKill) (Variables|Default|GetLifetime)))

(event Collision|EventActorBeginOverlap
  (params (OtherActor :type Actor%20Object%20Reference))
  (|CallParentFunction OtherActor) ; This node is disabled and will not be called.\nDrag off pins to build functionality.
)

(event EventCollisionBehavior
  (params (Location :type Vector :default "0, 0, 0") (DamagedActor :type Actor%20Object%20Reference) (HitComponent :type Primitive%20Component%20Object%20Reference))
  (Variables|/Script/Engine.MovementComponent|SetVelocity (Variables|Default|GetProjectileMovement) "0, 0, 0")
  (bind _size (Timeline|Growth Play)
    (:Update
      (Transformation|SetWorldScale3D (Variables|Default|GetSphere) (Math|Conversions|ToVector(Float) (* _size 5e+01))))
    (:Finished
      (bind _outactors (Actor|GetAllActorsOfClass "/Game/Characters/Enemies/BP_Enemy_Base.BP_Enemy_Base_C"))
      (for _array_element _outactors
        (Class|BPIDamagable|TakeDamage(Message) _array_element (Utilities|Struct|MakeS_DamageInfo 5e+03 "NewEnumerator2" "NewEnumerator0" false false false true 0.0 false 0 0))
        (Class|AISenseDamage|ReportDamageEvent 0 (Components|GetOwner) (Variables|Default|GetDamage) "0, 0, 0" "0, 0, 0" "None"))
      (bind _size_2 (Timeline|Growth2 Play)
        (:Update
          (Transformation|SetWorldScale3D (Variables|Default|GetSphere1) (Math|Conversions|ToVector(Float) (* _size_2 5e+01))))))))

(fn ConstructionScript
  (|CallParentFunction))