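; Devastation bullet that swallows another non-piercing projectile it overlaps and carries it hidden as a payload.
; The absorbed bullet is attached to the collider and stopped; hits and bounces trigger its collision behavior alongside Devastation's damage, with optional player and enemy phasing on overlap.
; Tick handles owner-following bullet-field movement, spiral offsets and acceleration.
; Bounces also call clustering, and lifetime expiry bursts both bullets unless deletion is cancelled.
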(event OnProjectileBounce(ProjectileMovement)
  (params (ImpactResult :type Hit%20Result%20Structure%20%28by%20ref%29) (ImpactVelocity :type Vector%20%28by%20ref%29 :default "0, 0, 0"))
  (CallFunction|DevastationCollision (.impactpoint ImpactResult))
  (CallFunction|DoCluster (.normal ImpactResult) (.hitactor ImpactResult) (Transformation|GetWorldLocation (Variables|Default|GetCollider))))

(event OnComponentBeginOverlap(Collider)
  (params (OverlappedComponent :type Primitive%20Component%20Object%20Reference) (OtherActor :type Actor%20Object%20Reference) (OtherComp :type Primitive%20Component%20Object%20Reference) (OtherBodyIndex :type Integer) (bFromSweep :type Boolean) (SweepResult :type Hit%20Result%20Structure%20%28by%20ref%29))
  (if (not (Variables|Default|GetStasis))
    (CallFunction|AbsorborCollide OtherActor)))

(event Custom|DevastationCollision
  (params (Location :type Vector) (DamagedActor :type Actor%20Object%20Reference))
  (bind _innerbullet (Variables|Default|GetInnerBullet))
  (Utilities|IsValid _innerbullet
    (:Is%20Valid
      (Default|CollisionBehavior _innerbullet (Transformation|GetWorldLocation (Variables|Default|GetCollider)) DamagedActor))
    (:Is%20Not%20Valid
      _))
  (Utilities|Casting|CastToBPI_Damagable DamagedActor)
  (CallFunction|DealDamage DamagedActor true))

(event EventBeginPlay
  (|CallParentFunction) ; This node is disabled and will not be called.\nDrag off pins to build functionality.
)

(event EventKillEventually
  (bind _innerbullet (Variables|Default|GetInnerBullet))
  (Utilities|FlowControl|Delay (Variables|Default|GetLifetime))
  (if (not (Variables|Default|GetCancelDeletion))
    (CallFunction|DoBurst (Transformation|GetWorldLocation (Variables|Default|GetCollider)))
    (Utilities|IsValid _innerbullet
      (:Is%20Valid
        (Default|DoBurst _innerbullet (Transformation|GetWorldLocation (Variables|/Game/Weapons/Bullets/Bullets/BP_ProjectileBase.BP_ProjectileBase_C|GetCollider _innerbullet)))
        (Actor|DestroyActor _innerbullet)
        (Actor|DestroyActor))
      (:Is%20Not%20Valid
        (Actor|DestroyActor)))))

(event EventTick
  (params (DeltaSeconds :type Float%20%28single-precision%29))
  (bind _returnvalue (Components|GetOwner))
  (bind _projectilemovement (Variables|Default|GetProjectileMovement))
  (bind _spiral (Variables|Default|GetSpiral))
  (if (Variables|Default|GetBulletField)
    (if (Utilities|IsValid _returnvalue)
      (Transformation|SetWorldLocation (Variables|Default|GetCollider) (+ (Transformation|GetActorLocation _returnvalue) (Variables|Default|GetOffset)) true false)
      (if (== (Variables|Default|GetSpiral) 0.0) :!label _label
        _
        (else
          (Variables|Default|SetTotalSeconds (+ (Variables|Default|GetTotalSeconds) DeltaSeconds))
          (Transformation|AddRelativeLocation (Variables|Default|GetCollider) (Math|Vector|MakeVector 0.0 (* (Math|Trig|Cos(Radians) (* (+ (Variables|Default|GetTotalSeconds) DeltaSeconds) (/ (Variables|Default|GetVelocity) 2e+02))) _spiral) (* (Math|Trig|Sin(Radians) (* (+ (Variables|Default|GetTotalSeconds) DeltaSeconds) (/ (Variables|Default|GetVelocity) 2e+02))) _spiral)) false false)))
      (if (not (== (Variables|Default|GetAcceleration) 1.0))
        (if (> (Math|Vector|VectorLength (Variables|/Script/Engine.MovementComponent|GetVelocity _projectilemovement)) 5e+01)
          (Variables|/Script/Engine.MovementComponent|SetVelocity _projectilemovement (+ (Variables|/Script/Engine.MovementComponent|GetVelocity _projectilemovement) (* (Variables|Default|GetAcceleration) DeltaSeconds (Math|Vector|Normalize (Variables|/Script/Engine.MovementComponent|GetVelocity _projectilemovement) 0.0))))
          (else
            (Variables|/Script/Engine.MovementComponent|SetVelocity (Variables|Default|GetProjectileMovement) "0, 0, 0")
            (if (or (Variables|Default|GetBulletField) (!= (Variables|Default|GetSpiral) 0.0))
              (Variables|Default|SetAcceleration 1.0)
              (else
                (Actor|Tick|SetActorTickEnabled false))))))
      (else
        (Actor|DestroyActor)))
    (else
      (goto _label))))

(event Collision|EventActorBeginOverlap
  (params (OtherActor :type Actor%20Object%20Reference))
  (|CallParentFunction OtherActor) ; This node is disabled and will not be called.\nDrag off pins to build functionality.
)

(event EventAbsorborCollide
  (params (Actor :type Actor%20Object%20Reference))
  (bind _asbp_projectile_base (Utilities|Casting|CastToBP_ProjectileBase Actor)
    (:then
      (Collision|SetCollisionResponsetoChannel (Variables|Default|GetCollider) "ECC_GameTraceChannel2" "ECR_Ignore")
      (Utilities|IsValid (Variables|Default|GetInnerBullet)
        (:Is%20Not%20Valid
          (if (not (>= (Variables|/Game/Weapons/Bullets/Bullets/BP_ProjectileBase.BP_ProjectileBase_C|GetPiercing _asbp_projectile_base) 1))
            (Collision|SetCollisionEnabled (Variables|/Game/Weapons/Bullets/Bullets/BP_ProjectileBase.BP_ProjectileBase_C|GetCollider _asbp_projectile_base) "NoCollision")
            (bind _output_get (Variables|Default|SetInnerBullet _asbp_projectile_base))
            (Actor|SetOwner _output_get 0)
            (Rendering|SetVisibility (Variables|/Game/Weapons/Bullets/Bullets/BP_ProjectileBase.BP_ProjectileBase_C|GetScene _output_get) false true)
            (Variables|/Game/Weapons/Bullets/Bullets/BP_ProjectileBase.BP_ProjectileBase_C|SetPiercing _output_get 2)
            (Variables|/Game/Weapons/Bullets/Bullets/BP_ProjectileBase.BP_ProjectileBase_C|SetDoPhysicsCalculation _asbp_projectile_base true)
            (Variables|/Script/Engine.ProjectileMovementComponent|SetProjectileGravityScale (Variables|/Game/Weapons/Bullets/Bullets/BP_ProjectileBase.BP_ProjectileBase_C|GetProjectileMovement _output_get) 0.0)
            (Variables|/Game/Weapons/Bullets/Bullets/BP_ProjectileBase.BP_ProjectileBase_C|SetCancelDeletion _output_get true)
            (Transformation|AttachComponentToComponent (Variables|/Game/Weapons/Bullets/Bullets/BP_ProjectileBase.BP_ProjectileBase_C|GetCollider _output_get) (Variables|Default|GetCollider) "None" "KeepWorld" "KeepWorld" "KeepWorld" true)
            (Game|Components|ProjectileMovement|SetVelocityinLocalSpace (Variables|/Game/Weapons/Bullets/Bullets/BP_ProjectileBase.BP_ProjectileBase_C|GetProjectileMovement _output_get) "0, 0, 0")))))
    (:CastFailed
      (if (Variables|Default|GetPhasePlayer)
        (Utilities|Casting|CastToBP_Player Actor
          (:CastFailed
            _)))
      (if (Variables|Default|GetPhaseEnemies)
        (Utilities|Casting|CastToBP_Enemy_Base Actor
          (:CastFailed
            _)))
      (CallFunction|DevastationCollision (Transformation|GetActorLocation) Actor))))

(fn ConstructionScript
  (|CallParentFunction))