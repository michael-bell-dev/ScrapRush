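; BP_Blaze is a bullet that explodes when its lifetime expires or it is killed.
; KillEventually waits out the lifetime and, unless deletion is cancelled, joins KillNow in triggering CollisionBehavior at the collider before destroying the actor.
; CollisionBehavior spawns a radius-scaled grenade explosion with sound, runs a temporary in-range attack, then calls EndOfLife.
; An InstantActivate branch that adds the owner to DamageArray is left unconnected.
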(event EventCollisionBehavior
  (params (Location :type Vector :default "0, 0, 0") (DamagedActor :type Actor%20Object%20Reference) (HitComponent :type Primitive%20Component%20Object%20Reference))
  (Effects|SpawnEmitteratLocation "/Game/Weapons/MilitaryWeapSilver/FX/P_Grenade_Explosion_01.P_Grenade_Explosion_01" Location "0, 0, 0" (Math|Conversions|ToVector(Float) (/ (Variables|Default|GetRadius) 3e+02)) true "AutoRelease")
  (Audio|PlaySoundatLocation "/Game/StarterContent/Audio/Explosion_Cue.Explosion_Cue" Location "0, 0, 0" 1.0 1.0 0.0 0 0 0 0)
  (CallFunction|TEMPORARYAttackinRange)
  (CallFunction|EndOfLife DamagedActor))

(event EventKillEventually
  (Utilities|FlowControl|Delay (Variables|Default|GetLifetime))
  (if (not (Variables|Default|GetCancelDeletion))
    (CallFunction|CollisionBehavior (Transformation|GetWorldLocation (Variables|Default|GetCollider)))
    (Actor|DestroyActor)))

(event EventKillNow
  (CallFunction|CollisionBehavior (Transformation|GetWorldLocation (Variables|Default|GetCollider)))
  (Actor|DestroyActor))

(fn ConstructionScript
  (|CallParentFunction))