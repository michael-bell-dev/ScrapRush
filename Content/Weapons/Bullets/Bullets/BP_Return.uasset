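; BP_Return is a bullet that teleports its owner to its location when killed or when its lifetime ends uncancelled.
; A MapDetection overlap test against Master_Room gates the direct teleport.
; If that fails, it traces back toward the owner, trying points offset behind each hit that lie in a room, unless the player's TeleportAnywhere waives this.
; It notifies BP_Player, then bursts and destroys itself, with collision handlers overridden empty.
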(event OnComponentBeginOverlap(Collider)
  (params (OverlappedComponent :type Primitive%20Component%20Object%20Reference) (OtherActor :type Actor%20Object%20Reference) (OtherComp :type Primitive%20Component%20Object%20Reference) (OtherBodyIndex :type Integer) (bFromSweep :type Boolean) (SweepResult :type Hit%20Result%20Structure%20%28by%20ref%29)))

(event EventBeginPlay
  (|CallParentFunction))

(event Collision|EventActorBeginOverlap
  (params (OtherActor :type Actor%20Object%20Reference)))

(event EventKillNow
  (bind _returnvalue (Components|GetOwner))
  (bind _collider (Variables|Default|GetCollider))
  (bind _returnvalue_2 (Transformation|GetWorldLocation _collider))
  (bind _returnvalue_3 (Transformation|GetActorRotation _returnvalue))
  (bind _asbp_player (Utilities|Casting|CastToBP_Player (Components|GetOwner))
    (:then
      (Default|PlayerTeleported _asbp_player)
      (Variables|Default|SetTeleport%20Anywhere (Variables|/Game/Characters/Player/BP_Player.BP_Player_C|GetTeleportAnywhere _asbp_player)))
    (:CastFailed
      _))
  (Transformation|SetWorldLocation (Variables|Default|GetMapDetection) "0, 0, 0" false true)
  (if (== (Utilities|Array|Length (Collision|GetOverlappingActors (Variables|Default|GetMapDetection) "/Game/Rooms/Rooms/Master_Room.Master_Room_C" :!class /Script/Engine.PrimitiveComponent)) 0)
    (bind _outhits (Class|KismetSystemLibrary|LineTraceMultiforObjects _returnvalue_2 (Transformation|GetActorLocation _returnvalue) (Utilities|Array|MakeArray "ObjectTypeQuery7" "ObjectTypeQuery2" "ObjectTypeQuery3" "ObjectTypeQuery4" "ObjectTypeQuery1" "ObjectTypeQuery6" "ObjectTypeQuery5") false 0 "None" true :!label _label))
    (bind _array_element (Utilities|Array|ForEachLoopwithBreak _outhits :!label _label_2)
      (:LoopBody
        (Transformation|SetWorldLocation (Variables|Default|GetMapDetection) (+ (.location _array_element) (* (Math|Vector|GetForwardVector (Variables|Default|GetCollider)) -1e+02)) false true)
        (if (Variables|Default|GetTeleport%20Anywhere)
          (bind _returnvalue_4 (Transformation|Teleport (Components|GetOwner) (+ (.location _array_element) (* (Math|Vector|GetForwardVector (Variables|Default|GetCollider)) -1e+02)) _returnvalue_3 :!label _label_3))
          (if _returnvalue_4
            (bind _asbp_player_2 (Utilities|Casting|CastToBP_Player (Components|GetOwner)))
            (Default|PlayerTeleported _asbp_player_2)
            (goto _label_2 Break))
          (elif (not (== (Utilities|Array|Length (Collision|GetOverlappingActors (Variables|Default|GetMapDetection) "/Game/Rooms/Rooms/Master_Room.Master_Room_C" :!class /Script/Engine.PrimitiveComponent)) 0))
            (goto _label_3))))
      (:Completed
        (Utilities|FlowControl|DelayUntilNextTick :!label _label_4)
        (CallFunction|DoBurst (Transformation|GetWorldLocation (Variables|Default|GetCollider)))
        (Actor|DestroyActor)))
    (else
      (bind _returnvalue_5 (Transformation|Teleport _returnvalue _returnvalue_2 _returnvalue_3))
      (if _returnvalue_5
        (bind _asbp_player_3 (Utilities|Casting|CastToBP_Player (Components|GetOwner))
          (:then
            (Default|PlayerTeleported _asbp_player_3)
            (goto _label_4))
          (:CastFailed
            (goto _label_4)))
        (else
          (goto _label))))))

(event EventCollisionBehavior
  (params (Location :type Vector :default "0, 0, 0") (DamagedActor :type Actor%20Object%20Reference) (HitComponent :type Primitive%20Component%20Object%20Reference)))

(event EventKillEventually
  (bind _returnvalue (Components|GetOwner))
  (bind _collider (Variables|Default|GetCollider))
  (bind _returnvalue_2 (Transformation|GetWorldLocation _collider))
  (bind _returnvalue_3 (Transformation|GetActorRotation _returnvalue))
  (Utilities|FlowControl|Delay (Variables|Default|GetLifetime))
  (if (not (Variables|Default|GetCancelDeletion))
    (bind _asbp_player (Utilities|Casting|CastToBP_Player (Components|GetOwner))
      (:then
        (Default|PlayerTeleported _asbp_player)
        (Variables|Default|SetTeleport%20Anywhere (Variables|/Game/Characters/Player/BP_Player.BP_Player_C|GetTeleportAnywhere _asbp_player)))
      (:CastFailed
        _))
    (Transformation|SetWorldLocation (Variables|Default|GetMapDetection) "0, 0, 0" false true)
    (if (== (Utilities|Array|Length (Collision|GetOverlappingActors (Variables|Default|GetMapDetection) "/Game/Rooms/Rooms/Master_Room.Master_Room_C" :!class /Script/Engine.PrimitiveComponent)) 0)
      (bind _outhits (Class|KismetSystemLibrary|LineTraceMultiforObjects _returnvalue_2 (Transformation|GetActorLocation _returnvalue) (Utilities|Array|MakeArray "ObjectTypeQuery7" "ObjectTypeQuery2" "ObjectTypeQuery3" "ObjectTypeQuery4" "ObjectTypeQuery1" "ObjectTypeQuery6" "ObjectTypeQuery5") false 0 "None" true :!label _label))
      (bind _array_element (Utilities|Array|ForEachLoopwithBreak _outhits :!label _label_2)
        (:LoopBody
          (Transformation|SetWorldLocation (Variables|Default|GetMapDetection) (+ (.location _array_element) (* (Math|Vector|GetForwardVector (Variables|Default|GetCollider)) -1e+02)) false true)
          (if (Variables|Default|GetTeleport%20Anywhere)
            (bind _returnvalue_4 (Transformation|Teleport (Components|GetOwner) (+ (.location _array_element) (* (Math|Vector|GetForwardVector (Variables|Default|GetCollider)) -1e+02)) _returnvalue_3 :!label _label_3))
            (if _returnvalue_4
              (bind _asbp_player_2 (Utilities|Casting|CastToBP_Player (Components|GetOwner)))
              (Default|PlayerTeleported _asbp_player_2)
              (goto _label_2 Break))
            (elif (not (== (Utilities|Array|Length (Collision|GetOverlappingActors (Variables|Default|GetMapDetection) "/Game/Rooms/Rooms/Master_Room.Master_Room_C" :!class /Script/Engine.PrimitiveComponent)) 0))
              (goto _label_3))))
        (:Completed
          (Utilities|FlowControl|DelayUntilNextTick :!label _label_4)
          (CallFunction|DoBurst (Transformation|GetWorldLocation (Variables|Default|GetCollider)))
          (Actor|DestroyActor)))
      (else
        (bind _returnvalue_5 (Transformation|Teleport _returnvalue _returnvalue_2 _returnvalue_3))
        (if _returnvalue_5
          (bind _asbp_player_3 (Utilities|Casting|CastToBP_Player (Components|GetOwner))
            (:then
              (Default|PlayerTeleported _asbp_player_3)
              (goto _label_4))
            (:CastFailed
              (goto _label_4)))
          (else
            (goto _label)))))))

(fn ConstructionScript
  (|CallParentFunction))