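; BP_Flame is a flame projectile that deals blockable damage to damageable actors it collides with.
; One tick after BeginPlay it either scales its velocity to launch or, when InstantActivate is set, stops moving.
; An instant flame with Stasis also attaches to the barrel socket of its owning player's or gunhead enemy's weapon.
; Instant flames never damage their owner.
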(event EventBeginPlay
  (bind _returnvalue (Components|GetOwner))
  (bind _projectilemovement (Variables|Default|GetProjectileMovement))
  (|CallParentFunction)
  (Utilities|FlowControl|DelayUntilNextTick)
  (if (Variables|Default|GetInstantActivate)
    (Variables|/Script/Engine.MovementComponent|SetVelocity (Variables|Default|GetProjectileMovement) "0, 0, 0")
    (if (Variables|Default|GetStasis)
      (bind _asbp_player (Utilities|Casting|CastToBP_Player _returnvalue)
        (:then
          (Transformation|AttachComponentToComponent (Variables|/Script/Engine.Actor|GetRootComponent (Variables|/Game/Characters/Player/BP_Player.BP_Player_C|GetCurrentWeapon _asbp_player)) "barrel" "KeepWorld" "KeepWorld" "KeepWorld" true))
        (:CastFailed
          (bind _asbp_enemy_gunhead_base (Utilities|Casting|CastToBP_EnemyGunhead_Base _returnvalue))
          (Transformation|AttachComponentToComponent (Variables|/Script/Engine.Actor|GetRootComponent (Variables|/Game/Characters/Enemies/BP_Enemy_Base.BP_Enemy_Base_C|GetWeapon _asbp_enemy_gunhead_base)) "barrel" "KeepWorld" "KeepWorld" "KeepWorld" true))))
    (else
      (Variables|/Script/Engine.MovementComponent|SetVelocity _projectilemovement (* (Variables|/Script/Engine.MovementComponent|GetVelocity _projectilemovement) 3e+03)))))

(event EventCollisionBehavior
  (params (Location :type Vector :default "0, 0, 0") (DamagedActor :type Actor%20Object%20Reference) (HitComponent :type Primitive%20Component%20Object%20Reference))
  (if (not (and (Variables|Default|GetInstantActivate) (== DamagedActor (Components|GetOwner))))
    (Utilities|Casting|CastToBPI_Damagable DamagedActor)
    (CallFunction|DealDamage DamagedActor true)))

(fn ConstructionScript
  (|CallParentFunction))