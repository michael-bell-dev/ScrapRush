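; BP_Ice is an ice bullet that damages and freezes the actor it hits.
; Its collision event deals blockable damage to damageable actors, then calls Freeze on enemies or players.
; Freeze reuses the bullet's Lifetime as duration and Damage as strength rather than separate freeze settings.
; Every collision finishes with EndOfLife, whether or not the target is damageable.
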(event EventCollisionBehavior
  (params (Location :type Vector :default "0, 0, 0") (DamagedActor :type Actor%20Object%20Reference) (HitComponent :type Primitive%20Component%20Object%20Reference))
  (bind _lifetime (Variables|Default|GetLifetime))
  (bind _damage (Variables|Default|GetDamage))
  (Utilities|Casting|CastToBPI_Damagable DamagedActor
    (:then
      (CallFunction|DealDamage DamagedActor true)
      (bind _asbp_enemy_base (Utilities|Casting|CastToBP_Enemy_Base DamagedActor)
        (:then
          (Default|Freeze _asbp_enemy_base _lifetime _damage))
        (:CastFailed
          (bind _asbp_player (Utilities|Casting|CastToBP_Player DamagedActor)
            (:then
              (Default|Freeze _asbp_player _lifetime _damage))
            (:CastFailed
              _)))))
    (:CastFailed
      _))
  (CallFunction|EndOfLife DamagedActor))

(fn ConstructionScript
  (|CallParentFunction))