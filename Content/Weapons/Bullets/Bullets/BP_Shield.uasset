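; Shield bullet that, on collision, raises a ring of three ShieldObject segments around the hit Character's base or the impact location.
; Segments sit 120 degrees apart relative to a forward vector, with scale, lifetime and health derived from the bullet's Radius, Lifetime and Damage.
; If the third segment is valid, damageable targets also take blockable damage.
; Piercing bullets briefly disable overlaps then continue; others are destroyed.
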(event EventCollisionBehavior
  (params (Location :type Vector :default "0, 0, 0") (DamagedActor :type Actor%20Object%20Reference) (HitComponent :type Primitive%20Component%20Object%20Reference))
  (bind _damage (Variables|Default|GetDamage))
  (bind _radius (Variables|Default|GetRadius))
  (bind _radius_2 (Variables|Default|GetRadius))
  (bind _radius_3 (Variables|Default|GetRadius))
  (bind _returnvalue (/ _radius_2 1.8e+02))
  (bind _returnvalue_2 (/ _radius 1.8e+02))
  (bind _returnvalue_3 (* _damage 2.0))
  (bind _returnvalue_4 (/ _radius_3 1.8e+02))
  (Variables|/Script/Engine.PrimitiveComponent|SetbGenerateOverlapEvents (Variables|Default|GetCollider) false)
  (Utilities|Casting|CastToCharacter DamagedActor
    (:then
      (Variables|Default|SetOwnerLocation (- (Transformation|GetActorLocation DamagedActor) "0.000000,0.000000,110.000000"))
      (Variables|Default|SetOwnerForward (Transformation|GetActorForwardVector DamagedActor)))
    (:CastFailed
      (Variables|Default|SetOwnerLocation Location)
      (Variables|Default|SetOwnerForward (Math|Vector|Normalize (* (Transformation|GetActorForwardVector) "1.000000,1.000000,0.000000") 0.0))))
  (bind _returnvalue_5 (Game|SpawnActorfromClass "/Game/Weapons/Bullets/Bullets/ShieldObject.ShieldObject_C" (Math|Transform|MakeTransform (+ (Variables|Default|GetOwnerLocation) (* (Math|Vector|RotateVectorAroundAxis (Variables|Default|GetOwnerForward) -19.0 "0.000000,0.000000,1.000000") _radius)) (Math|Rotator|MakeRotator 0.0 0.0 (+ (.yaw (Math|Rotator|MakeRotfromX (Variables|Default|GetOwnerForward))) 2e+02)) (Math|Vector|MakeVector _returnvalue_2 _returnvalue_2 1.3)) "Undefined" "MultiplyWithRoot" 0 0))
  (Variables|/Game/Weapons/Bullets/Bullets/ShieldObject.ShieldObject_C|Set"radius" _returnvalue_5 (Variables|Default|GetRadius))
  (Utilities|IsValid _returnvalue_5
    (:Is%20Valid
      (Default|SetLife _returnvalue_5 (* (Variables|Default|GetLifetime) 5.0))
      (Variables|/Game/Weapons/Bullets/Bullets/ShieldObject.ShieldObject_C|SetMaxHealth _returnvalue_5 _returnvalue_3)
      (Variables|/Game/Weapons/Bullets/Bullets/ShieldObject.ShieldObject_C|SetHealth _returnvalue_5 _returnvalue_3))
    (:Is%20Not%20Valid
      _))
  (bind _returnvalue_6 (Game|SpawnActorfromClass "/Game/Weapons/Bullets/Bullets/ShieldObject.ShieldObject_C" (Math|Transform|MakeTransform (+ (Variables|Default|GetOwnerLocation) (* (Math|Vector|RotateVectorAroundAxis (Variables|Default|GetOwnerForward) -139.0 "0.000000,0.000000,1.000000") _radius_3)) (Math|Rotator|MakeRotator 0.0 0.0 (+ (.yaw (Math|Rotator|MakeRotfromX (Variables|Default|GetOwnerForward))) 8e+01)) (Math|Vector|MakeVector _returnvalue_4 _returnvalue_4 1.3)) "Undefined" "MultiplyWithRoot" 0 0))
  (Variables|/Game/Weapons/Bullets/Bullets/ShieldObject.ShieldObject_C|Set"radius" _returnvalue_6 (Variables|Default|GetRadius))
  (Utilities|IsValid _returnvalue_6
    (:Is%20Valid
      (Default|SetLife _returnvalue_6 (* (Variables|Default|GetLifetime) 5.0))
      (Variables|/Game/Weapons/Bullets/Bullets/ShieldObject.ShieldObject_C|SetMaxHealth _returnvalue_6 _returnvalue_3)
      (Variables|/Game/Weapons/Bullets/Bullets/ShieldObject.ShieldObject_C|SetHealth _returnvalue_6 _returnvalue_3))
    (:Is%20Not%20Valid
      _))
  (bind _returnvalue_7 (Game|SpawnActorfromClass "/Game/Weapons/Bullets/Bullets/ShieldObject.ShieldObject_C" (Math|Transform|MakeTransform (+ (Variables|Default|GetOwnerLocation) (* (Math|Vector|RotateVectorAroundAxis (Variables|Default|GetOwnerForward) 101.0 "0.000000,0.000000,1.000000") _radius_2)) (Math|Rotator|MakeRotator 0.0 0.0 (+ (.yaw (Math|Rotator|MakeRotfromX (Variables|Default|GetOwnerForward))) 3.2e+02)) (Math|Vector|MakeVector _returnvalue _returnvalue 1.3)) "Undefined" "MultiplyWithRoot" 0 0))
  (Variables|/Game/Weapons/Bullets/Bullets/ShieldObject.ShieldObject_C|Set"radius" _returnvalue_7 (Variables|Default|GetRadius))
  (Utilities|IsValid _returnvalue_7
    (:Is%20Valid
      (Default|SetLife _returnvalue_7 (* (Variables|Default|GetLifetime) 5.0))
      (Variables|/Game/Weapons/Bullets/Bullets/ShieldObject.ShieldObject_C|SetMaxHealth _returnvalue_7 _returnvalue_3)
      (Variables|/Game/Weapons/Bullets/Bullets/ShieldObject.ShieldObject_C|SetHealth _returnvalue_7 _returnvalue_3)
      (Utilities|Casting|CastToBPI_Damagable DamagedActor
        (:then
          (CallFunction|DealDamage DamagedActor true))
        (:CastFailed
          _)))
    (:Is%20Not%20Valid
      _))
  (if (>= (Variables|Default|GetPiercing) 1)
    (Utilities|FlowControl|Delay 0.1)
    (Variables|/Script/Engine.PrimitiveComponent|SetbGenerateOverlapEvents (Variables|Default|GetCollider) true)
    (else
      (Actor|DestroyActor))))

(fn ConstructionScript
  (|CallParentFunction))

(fn CustomStasis
  (Variables|Default|SetOwnerForward (Math|Vector|Normalize (* (Transformation|GetActorForwardVector) "1.000000,1.000000,0.000000") 0.0)))