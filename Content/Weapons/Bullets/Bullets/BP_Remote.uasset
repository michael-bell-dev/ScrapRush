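; BP_Remote is a projectile that acts as a remote trigger for the player's other shots when it collides.
; On collision it deals blockable damage to damagable actors, then gathers every BP_ProjectileBase in the level, excluding BP_Remote instances to avoid triggering its own kind.
; Each player-owned projectile loses one Piercing, bursts and runs its own collision behavior at its current position.
; The remote then ends its life.
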(event EventCollisionBehavior
  (params (Location :type Vector :default "0, 0, 0") (DamagedActor :type Actor%20Object%20Reference) (HitComponent :type Primitive%20Component%20Object%20Reference))
  (Utilities|Casting|CastToBPI_Damagable DamagedActor
    (:then
      (CallFunction|DealDamage DamagedActor true))
    (:CastFailed
      _))
  (bind _outactors (Actor|GetAllActorsOfClass "/Game/Weapons/Bullets/Bullets/BP_ProjectileBase.BP_ProjectileBase_C"))
  (Variables|Default|SetOut%20Actors _outactors)
  (bind _outactors_2 (Actor|GetAllActorsOfClass "BP_Remote_C"))
  (for _array_element _outactors_2
    (Utilities|Array|RemoveItem (Variables|Default|GetOut%20Actors) _array_element))
  (for _array_element_2 (Variables|Default|GetOut%20Actors)
    (Utilities|Casting|CastToBP_Player (Components|GetOwner _array_element_2))
    (Math|Integer|DecrementInt (Variables|/Game/Weapons/Bullets/Bullets/BP_ProjectileBase.BP_ProjectileBase_C|GetPiercing _array_element_2)
      (:%20%20
        (Default|DoBurst _array_element_2 (Transformation|GetWorldLocation (Variables|/Game/Weapons/Bullets/Bullets/BP_ProjectileBase.BP_ProjectileBase_C|GetCollider _array_element_2)))
        (Default|CollisionBehavior _array_element_2 (Transformation|GetWorldLocation (Variables|/Game/Weapons/Bullets/Bullets/BP_ProjectileBase.BP_ProjectileBase_C|GetCollider _array_element_2))))))
  (CallFunction|EndOfLife DamagedActor))

(fn ConstructionScript
  (|CallParentFunction))