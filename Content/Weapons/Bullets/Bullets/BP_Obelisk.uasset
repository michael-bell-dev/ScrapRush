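; BP_Obelisk is a bullet that spawns an obelisk object where it hits and damages damageable victims with a blockable hit.
; On collision it spawns the obelisk at zero scale, lowered for character hits or aligned to the surface normal otherwise, deriving radius, life and health from bullet stats.
; It briefly disables overlaps and continues when piercing or lacking a valid hit actor, otherwise destroys itself.
; CustomStasis sets OwnerForward to the flattened forward vector.
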(event EventCollisionBehavior
  (params (Location :type Vector :default "0, 0, 0") (DamagedActor :type Actor%20Object%20Reference) (HitComponent :type Primitive%20Component%20Object%20Reference))
  (bind _damage (Variables|Default|GetDamage))
  (bind _returnvalue (* _damage 2.0))
  (Variables|/Script/Engine.PrimitiveComponent|SetbGenerateOverlapEvents (Variables|Default|GetCollider) false)
  (Utilities|Casting|CastToCharacter DamagedActor
    (:then
      (Variables|Default|SetSpawn%20Transform%20Location (Math|Vector|MakeVector (.x Location) (.y Location) (- (.z Location) 1.2e+02))))
    (:CastFailed
      (Variables|Default|SetSpawn%20Transform%20Rotation (Math|Rotator|MakeRotfromZ (Variables|Default|GetNormal)))
      (Variables|Default|SetSpawn%20Transform%20Location (Math|Vector|MakeVector (.x Location) (.y Location) (.z Location)))))
  (bind _returnvalue_2 (Game|SpawnActorfromClass "/Game/Weapons/Bullets/Bullets/ObeliskObject.ObeliskObject_C" (Math|Transform|MakeTransform (Variables|Default|GetSpawn%20Transform%20Location) (Variables|Default|GetSpawn%20Transform%20Rotation) "0.0,0.0,0.0") "Undefined" "MultiplyWithRoot" 0 0))
  (Utilities|IsValid _returnvalue_2
    (:Is%20Valid
      (Variables|/Game/Weapons/Bullets/Bullets/ObeliskObject.ObeliskObject_C|Set"radius" _returnvalue_2 (* (Variables|Default|GetRadius) 4.0))
      (Default|SetLife _returnvalue_2 (* (Variables|Default|GetLifetime) 5.0))
      (Variables|/Game/Weapons/Bullets/Bullets/ObeliskObject.ObeliskObject_C|SetMaxHealth _returnvalue_2 _returnvalue)
      (Variables|/Game/Weapons/Bullets/Bullets/ObeliskObject.ObeliskObject_C|SetHealth _returnvalue_2 _returnvalue)
      (Utilities|Casting|CastToBPI_Damagable DamagedActor
        (:then
          (CallFunction|DealDamage DamagedActor true))
        (:CastFailed
          _)))
    (:Is%20Not%20Valid
      _))
  (if (or (>= (Variables|Default|GetPiercing) 1) (not (Utilities|IsValid DamagedActor)))
    (Utilities|FlowControl|Delay 0.1)
    (Variables|/Script/Engine.PrimitiveComponent|SetbGenerateOverlapEvents (Variables|Default|GetCollider) true)
    (else
      (Actor|DestroyActor))))

(fn ConstructionScript
  (|CallParentFunction))

(fn CustomStasis
  (Variables|Default|SetOwnerForward (Math|Vector|Normalize (* (Transformation|GetActorForwardVector) "1.000000,1.000000,0.000000") 0.0)))