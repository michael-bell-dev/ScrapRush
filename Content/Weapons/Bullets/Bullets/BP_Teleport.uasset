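; Teleport bullet that damages what it hits and moves its owner to the impact point, or to where it expires.
; MapDetection checks that the destination overlaps a Master_Room before teleporting.
; If that check or the teleport fails, a multi-trace back toward the owner tries backed-off hit points, skipping the room check when the player has TeleportAnywhere.
; Hitting the owner increments Piercing instead of dealing damage.
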(event EventKillEventually
  (Utilities|FlowControl|Delay (Variables|Default|GetLifetime))
  (if (not (Variables|Default|GetCancelDeletion))
    (CallFunction|CollisionBehavior (Transformation|GetWorldLocation (Variables|Default|GetCollider)))
    (CallFunction|DoBurst (Transformation|GetWorldLocation (Variables|Default|GetCollider)))
    (Actor|DestroyActor)))

(event EventCollisionBehavior
  (params (Location :type Vector :default "0, 0, 0") (DamagedActor :type Actor%20Object%20Reference) (HitComponent :type Primitive%20Component%20Object%20Reference))
  (bind _returnvalue (Components|GetOwner))
  (bind _returnvalue_2 (Transformation|GetActorRotation _returnvalue))
  (bind _asbp_player (Utilities|Casting|CastToBP_Player (Components|GetOwner))
    (:then
      (Default|PlayerTeleported _asbp_player)
      (Variables|Default|SetTeleport%20Anywhere (Variables|/Game/Characters/Player/BP_Player.BP_Player_C|GetTeleportAnywhere _asbp_player)))
    (:CastFailed
      _))
  (if (== DamagedActor (Components|GetOwner))
    (Math|Integer|IncrementInt (Variables|Default|GetPiercing)
      (:%20%20
        _))
    (else
      (Utilities|Casting|CastToBPI_Damagable DamagedActor
        (:then
          (CallFunction|DealDamage DamagedActor true))
        (:CastFailed
          _))))
  (Utilities|IsValid (Components|GetOwner)
    (:Is%20Valid
      (Transformation|SetWorldLocation (Variables|Default|GetMapDetection) Location false true)
      (if (== (Utilities|Array|Length (Collision|GetOverlappingActors (Variables|Default|GetMapDetection) "/Game/Rooms/Rooms/Master_Room.Master_Room_C" :!class /Script/Engine.PrimitiveComponent)) 0)
        (Development|PrintString (Utilities|GetDisplayName DamagedActor))
        (bind _outhits (Class|KismetSystemLibrary|LineTraceMultiforObjects Location (Transformation|GetActorLocation _returnvalue) (Utilities|Array|MakeArray "ObjectTypeQuery7" "ObjectTypeQuery2" "ObjectTypeQuery3" "ObjectTypeQuery4" "ObjectTypeQuery1" "ObjectTypeQuery6" "ObjectTypeQuery5") false 0 "None" true :!label _label))
        (bind _array_element (Utilities|Array|ForEachLoopwithBreak _outhits :!label _label_2)
          (:LoopBody
            (Transformation|SetWorldLocation (Variables|Default|GetMapDetection) (+ (.location _array_element) (* (Math|Vector|GetForwardVector (Variables|Default|GetCollider)) -1e+02)) false true)
            (if (Variables|Default|GetTeleport%20Anywhere)
              (bind _returnvalue_3 (Transformation|Teleport (Components|GetOwner) (+ (.location _array_element) (* (Math|Vector|GetForwardVector (Variables|Default|GetCollider)) -1e+02)) _returnvalue_2 :!label _label_3))
              (if _returnvalue_3
                (bind _asbp_player_2 (Utilities|Casting|CastToBP_Player (Components|GetOwner)))
                (Default|PlayerTeleported _asbp_player_2)
                (goto _label_2 Break))
              (elif (not (== (Utilities|Array|Length (Collision|GetOverlappingActors (Variables|Default|GetMapDetection) "/Game/Rooms/Rooms/Master_Room.Master_Room_C" :!class /Script/Engine.PrimitiveComponent)) 0))
                (goto _label_3))))
          (:Completed
            (CallFunction|EndOfLife DamagedActor :!label _label_4)))
        (else
          (bind _returnvalue_4 (Transformation|Teleport _returnvalue Location _returnvalue_2))
          (if _returnvalue_4
            (bind _asbp_player_3 (Utilities|Casting|CastToBP_Player (Components|GetOwner))
              (:then
                (Default|PlayerTeleported _asbp_player_3)
                (goto _label_4))
              (:CastFailed
                (goto _label_4)))
            (else
              (goto _label))))))
    (:Is%20Not%20Valid
      (Actor|DestroyActor))))

(fn ConstructionScript
  (|CallParentFunction))