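; BP_Rocket is an explosive projectile that builds on inherited bullet logic.
; On capsule overlap it waits a tick if its values are not updated, then handles piercing, stasis, knockback and clustering before triggering its collision behavior.
; That behavior damages damageable targets, spawns a radius-scaled explosion with sound and AI noise, runs a temporary in-range attack and ends the rocket's life.
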(event OnComponentBeginOverlap(Capsule)
  (params (OverlappedComponent :type Primitive%20Component%20Object%20Reference) (OtherActor :type Actor%20Object%20Reference) (OtherComp :type Primitive%20Component%20Object%20Reference) (OtherBodyIndex :type Integer) (bFromSweep :type Boolean) (SweepResult :type Hit%20Result%20Structure%20%28by%20ref%29))
  (bind _collider (Variables|Default|GetCollider))
  (bind _returnvalue (Transformation|GetWorldLocation _collider))
  (if (Variables|Default|GetValuesUpdated)
    _
    (else
      (Utilities|FlowControl|DelayUntilNextTick)))
  (if (< (Variables|Default|GetPiercing) 0)
    (Actor|DestroyActor)
    (elif (not (Variables|Default|GetStasis))
      (Math|Integer|DecrementInt (Variables|Default|GetPiercing)
        (:%20%20
          (if (== (Variables|Default|GetKnockback) 0.0)
            _
            (else
              (CallFunction|ApplyKnockback OtherActor OtherComp)))
          (CallFunction|DoCluster (.impactnormal SweepResult) OtherActor _returnvalue)
          (CallFunction|CollisionBehavior _returnvalue OtherActor OtherComp))))))

(event EventCollisionBehavior
  (params (Location :type Vector :default "0, 0, 0") (DamagedActor :type Actor%20Object%20Reference) (HitComponent :type Primitive%20Component%20Object%20Reference))
  (Utilities|Casting|CastToBPI_Damagable DamagedActor
    (:then
      (CallFunction|DealDamage DamagedActor true))
    (:CastFailed
      _))
  (Effects|SpawnEmitteratLocation "/Game/M5VFXVOL2/Particles/Explosion/Fire_Exp_00.Fire_Exp_00" Location "0, 0, 0" (Math|Conversions|ToVector(Float) (/ (Variables|Default|GetRadius) 3e+02)) true "AutoRelease")
  (Audio|PlaySoundatLocation "/Game/StarterContent/Audio/Explosion_Cue.Explosion_Cue" Location "0, 0, 0" 1.0 1.0 0.0 0 0 0 0)
  (Class|Actor|MakeNoise 1.0 0 Location 0.0 "None")
  (CallFunction|TEMPORARYAttackinRange)
  (CallFunction|EndOfLife))

(fn ConstructionScript
  (|CallParentFunction))