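; BP_Fix is a bullet that pulls what it hits to just in front of its owner.
; Its CollisionBehavior deals blockable damage to damageable actors, then sweeps them to a point along the owner's forward vector and calls EndOfLife.
; Pickups skip the damage but get the same pull.
; Any other valid hit destroys the bullet unless it has Piercing.
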(event EventCollisionBehavior
  (params (Location :type Vector :default "0, 0, 0") (DamagedActor :type Actor%20Object%20Reference) (HitComponent :type Primitive%20Component%20Object%20Reference))
  (bind _returnvalue (Components|GetOwner))
  (Utilities|Casting|CastToBPI_Damagable DamagedActor
    (:then
      (CallFunction|DealDamage DamagedActor true)
      (Utilities|IsValid DamagedActor :!label _label
        (:Is%20Valid
          (Transformation|SetActorLocation DamagedActor (+ (* (Transformation|GetActorForwardVector _returnvalue) 1e+02) (Transformation|GetActorLocation _returnvalue)) true false))
        (:Is%20Not%20Valid
          _))
      (CallFunction|EndOfLife DamagedActor))
    (:CastFailed
      (Utilities|Casting|CastToBP_PickupBase DamagedActor
        (:then
          (goto _label))
        (:CastFailed
          (if (not (or (>= (Variables|Default|GetPiercing) 1) (not (Utilities|IsValid DamagedActor))))
            (Actor|DestroyActor)))))))

(fn ConstructionScript
  (|CallParentFunction))