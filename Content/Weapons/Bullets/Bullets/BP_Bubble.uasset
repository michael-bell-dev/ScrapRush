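; Bubble projectile that deals damage and can swallow another projectile to carry along as a payload.
; On overlap, an empty bubble hides, freezes and attaches a non-piercing BP_ProjectileBase; other actors are filtered by stasis and phase modifiers.
; Damageable hits also trigger the inner bullet's collision behavior, releasing it unless the bubble pierces.
; Lifetime expiry also releases the payload, and bounces run collision plus cluster logic.
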(event OnProjectileBounce(ProjectileMovement)
  (params (ImpactResult :type Hit%20Result%20Structure%20%28by%20ref%29) (ImpactVelocity :type Vector%20%28by%20ref%29 :default "0, 0, 0"))
  (CallFunction|BubbleCollision (.impactpoint ImpactResult))
  (CallFunction|DoCluster (.normal ImpactResult) (.hitactor ImpactResult) (Transformation|GetWorldLocation (Variables|Default|GetCollider)) false))

(event OnComponentBeginOverlap(Collider)
  (params (OverlappedComponent :type Primitive%20Component%20Object%20Reference) (OtherActor :type Actor%20Object%20Reference) (OtherComp :type Primitive%20Component%20Object%20Reference) (OtherBodyIndex :type Integer) (bFromSweep :type Boolean) (SweepResult :type Hit%20Result%20Structure%20%28by%20ref%29))
  (CallFunction|AbsorborCollide OtherActor))

(event Custom|BubbleCollision
  (params (Location :type Vector) (DamagedActor :type Actor%20Object%20Reference))
  (bind _piercing (Variables|Default|GetPiercing))
  (bind _innerbullet (Variables|Default|GetInnerBullet))
  (bind _returnvalue (> _piercing 0))
  (Utilities|Casting|CastToBPI_Damagable DamagedActor)
  (CallFunction|DealDamage DamagedActor true)
  (Utilities|IsValid _innerbullet
    (:Is%20Valid
      (Default|CollisionBehavior _innerbullet Location DamagedActor)
      (if (not _returnvalue)
        (Collision|SetCollisionEnabled (Variables|/Game/Weapons/Bullets/Bullets/BP_ProjectileBase.BP_ProjectileBase_C|GetCollider _innerbullet) "QueryOnly")
        (Default|UnStatis _innerbullet)
        (CallFunction|EndOfLife DamagedActor :!label _label)))
    (:Is%20Not%20Valid
      (if (not _returnvalue)
        (goto _label)))))

(event Custom|AbsorbOrCollide
  (params (Actor :type Actor%20Object%20Reference))
  (bind _modifiers (Variables|Default|GetModifiers))
  (bind _asbp_projectile_base (Utilities|Casting|CastToBP_ProjectileBase Actor)
    (:then
      (Collision|SetCollisionResponsetoChannel (Variables|Default|GetCollider) "ECC_GameTraceChannel2" "ECR_Ignore")
      (Utilities|IsValid (Variables|Default|GetInnerBullet)
        (:Is%20Valid
          (if (not (>= (Variables|/Game/Weapons/Bullets/Bullets/BP_ProjectileBase.BP_ProjectileBase_C|GetPiercing _asbp_projectile_base) 1))
            (CallFunction|BubbleCollision (Transformation|GetActorLocation) Actor :!label _label)))
        (:Is%20Not%20Valid
          (if (not (>= (Variables|/Game/Weapons/Bullets/Bullets/BP_ProjectileBase.BP_ProjectileBase_C|GetPiercing _asbp_projectile_base) 1))
            (Collision|SetCollisionEnabled (Variables|/Game/Weapons/Bullets/Bullets/BP_ProjectileBase.BP_ProjectileBase_C|GetCollider _asbp_projectile_base) "NoCollision")
            (bind _output_get (Variables|Default|SetInnerBullet _asbp_projectile_base))
            (Actor|SetOwner _output_get 0)
            (Rendering|SetVisibility (Variables|/Game/Weapons/Bullets/Bullets/BP_ProjectileBase.BP_ProjectileBase_C|GetScene _output_get) false true)
            (Variables|/Game/Weapons/Bullets/Bullets/BP_ProjectileBase.BP_ProjectileBase_C|SetDoPhysicsCalculation _output_get true)
            (Variables|/Script/Engine.ProjectileMovementComponent|SetProjectileGravityScale (Variables|/Game/Weapons/Bullets/Bullets/BP_ProjectileBase.BP_ProjectileBase_C|GetProjectileMovement _output_get) 0.0)
            (Variables|/Game/Weapons/Bullets/Bullets/BP_ProjectileBase.BP_ProjectileBase_C|SetCancelDeletion _output_get true)
            (Transformation|AttachComponentToComponent (Variables|/Game/Weapons/Bullets/Bullets/BP_ProjectileBase.BP_ProjectileBase_C|GetCollider _output_get) (Variables|Default|GetCollider) "None" "KeepWorld" "KeepWorld" "KeepWorld" true)
            (Game|Components|ProjectileMovement|SetVelocityinLocalSpace (Variables|/Game/Weapons/Bullets/Bullets/BP_ProjectileBase.BP_ProjectileBase_C|GetProjectileMovement _output_get) "0, 0, 0")))))
    (:CastFailed
      (if (not (Variables|Default|GetStasis))
        (switch Utilities|FlowControl|Switch|SwitchonECollisionChannel "ECC_WorldStatic"
          (:ECC_WorldStatic
            _)
          (:ECC_WorldDynamic
            _)
          (:ECC_PhysicsBody
            _)
          (:ECC_Destructible
            _))
        (if (not (.phasewalls _modifiers))
          (if (.phaseenemies _modifiers)
            (Utilities|Casting|CastToCharacter Actor
              (:CastFailed
                (goto _label)))
            (elif (.phaseplayer _modifiers)
              (Utilities|Casting|CastToBP_Player Actor
                (:CastFailed
                  (goto _label)))
              (else
                (goto _label)))))))))

(event EventBeginPlay
  (|CallParentFunction)
  (if (< (Math|Float|Absolute(Float) (.gravity (Variables|Default|GetModifiers))) 0.3)
    (Variables|/Script/Engine.ProjectileMovementComponent|SetProjectileGravityScale (Variables|Default|GetProjectileMovement) 0.0))
  (Actor|Tick|SetActorTickEnabled true))

(event EventKillEventually
  (bind _echoloop (Variables|Default|GetEchoLoop))
  (bind _innerbullet (Variables|Default|GetInnerBullet))
  (Utilities|FlowControl|Delay (Variables|Default|GetLifetime))
  (if (not (Variables|Default|GetCancelDeletion))
    (Utilities|IsValid _innerbullet
      (:Is%20Valid
        (Default|UnStatis _innerbullet)
        (Collision|SetCollisionEnabled (Variables|/Game/Weapons/Bullets/Bullets/BP_ProjectileBase.BP_ProjectileBase_C|GetCollider _innerbullet) "QueryOnly"))
      (:Is%20Not%20Valid
        _))
    (if (Class|KismetSystemLibrary|TimerExistsHandle _echoloop)
      (Utilities|Time|InvalidateTimerHandle _echoloop))
    (CallFunction|DoKill)))

(event EventDestroyed
  (Actor|Tick|SetActorTickEnabled false))

(event Collision|EventActorBeginOverlap
  (params (OtherActor :type Actor%20Object%20Reference)))

(fn ConstructionScript
  (|CallParentFunction))