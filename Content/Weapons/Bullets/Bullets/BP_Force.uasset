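; BP_Force is a bullet Blueprint that sets off a radial impulse scaled by its damage.
; On collision it multiplies the RadialForce strengths by Damage, applies Radius, damages any BPI_Damagable actor with a blockable hit, then fires the impulse at that location and ends its life.
; If its lifetime expires without deletion being cancelled, it runs the same collision behavior at the collider's position and destroys itself.
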(event EventKillEventually
  (Utilities|FlowControl|Delay (Variables|Default|GetLifetime))
  (if (not (Variables|Default|GetCancelDeletion))
    (CallFunction|CollisionBehavior (Transformation|GetWorldLocation (Variables|Default|GetCollider)))
    (Actor|DestroyActor)))

(event EventCollisionBehavior
  (params (Location :type Vector :default "0, 0, 0") (DamagedActor :type Actor%20Object%20Reference) (HitComponent :type Primitive%20Component%20Object%20Reference))
  (bind _radialforce (Variables|Default|GetRadialForce))
  (Variables|/Script/Engine.RadialForceComponent|SetImpulseStrength _radialforce (* (Variables|/Script/Engine.RadialForceComponent|GetImpulseStrength (Variables|Default|GetRadialForce)) (Variables|Default|GetDamage)))
  (Variables|/Script/Engine.RadialForceComponent|SetForceStrength _radialforce (* (Variables|/Script/Engine.RadialForceComponent|GetForceStrength (Variables|Default|GetRadialForce)) (Variables|Default|GetDamage)))
  (Variables|/Script/Engine.RadialForceComponent|SetRadius _radialforce (Variables|Default|GetRadius))
  (Utilities|Casting|CastToBPI_Damagable DamagedActor
    (:then
      (CallFunction|DealDamage DamagedActor true))
    (:CastFailed
      _))
  (Transformation|SetWorldLocation (Variables|Default|GetRadialForce) Location false false)
  (Class|RadialForceComponent|FireImpulse (Variables|Default|GetRadialForce))
  (CallFunction|EndOfLife DamagedActor))

(fn ConstructionScript
  (|CallParentFunction))