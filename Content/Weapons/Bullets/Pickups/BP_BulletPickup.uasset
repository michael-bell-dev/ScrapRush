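; Bullet pickup the player interacts with to add its bullet type to their inventory, paying first if it is a shop item.
; DT_Bullet, keyed by the bullet type enum name, supplies the pickup material, price and spawn class.
; The bullet takes the first placeholder or unused slot; when full, it replaces slot 0, whose old bullet spawns in front of the player.
; The pickup then destroys itself.
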(event Custom|SetBulletMaterial
  (params (BulletType :type E_BulletTypes%20Enum :default "NewEnumerator21"))
  (bind _returnvalue (Utilities|GetDataTableRow "/Game/Characters/Player/Inventory/DataStructures/DT_Bullet.DT_Bullet" (Utilities|String|StringToName (Utilities|String|EnumtoString BulletType)))
    (:then
      (Rendering|Material|SetMaterial (Variables|Default|GetStaticMesh) 0 (.pickupmaterial _returnvalue))
      (Variables|Default|SetBulletType BulletType))))

(event EventBeginPlay
  (|CallParentFunction)
  (bind _returnvalue (Utilities|GetDataTableRow "/Game/Characters/Player/Inventory/DataStructures/DT_Bullet.DT_Bullet" (Utilities|String|StringToName (Utilities|String|EnumtoString (Variables|Default|GetBulletType))))
    (:then
      (Variables|Default|SetValue (.value _returnvalue)))))

(event EventInteract
  (params (Character%20Picking%20Up :type Actor%20Object%20Reference))
  (bind _value (Variables|Default|GetValue))
  (bind _asbp_player (Utilities|Casting|CastToBP_Player Character%20Picking%20Up))
  (if (Variables|Default|GetShopItem)
    (if (>= (Variables|/Game/Characters/Player/BP_Player.BP_Player_C|GetMoney _asbp_player) _value)
      (Variables|/Game/Characters/Player/BP_Player.BP_Player_C|SetMoney _asbp_player (- (Variables|/Game/Characters/Player/BP_Player.BP_Player_C|GetMoney _asbp_player) _value))
      (Variables|Default|SetInventoryHadRoom false :!label _label)
      (if (Variables|/Game/Characters/Player/BP_Player.BP_Player_C|GetFirstBulletPickup _asbp_player)
        (Default|FirstBullet (Variables|/Game/Characters/Player/BP_Player.BP_Player_C|GetMessageInteract _asbp_player)))
      (bind _index (Utilities|FlowControl|ForLoopwithBreak 0 32 :!label _label_2)
        (:LoopBody
          (if (Utilities|Array|IsValidIndex (Variables|/Game/Characters/Player/BP_Player.BP_Player_C|GetBulletInventory _asbp_player) _index)
            (if (Utilities|Enum|Equal(Enum) (Utilities|Array|Get(acopy) (Variables|/Game/Characters/Player/BP_Player.BP_Player_C|GetBulletInventory _asbp_player) _index) "NewEnumerator21")
              (Utilities|Array|SetArrayElem (Variables|/Game/Characters/Player/BP_Player.BP_Player_C|GetBulletInventory _asbp_player) _index (Variables|Default|GetBulletType) true)
              (Variables|Default|SetInventoryHadRoom true :!label _label_3)
              (goto _label_2 Break))
            (else
              (Utilities|Array|SetArrayElem (Variables|/Game/Characters/Player/BP_Player.BP_Player_C|GetBulletInventory _asbp_player) _index (Variables|Default|GetBulletType) true)
              (goto _label_3))))
        (:Completed
          (if (Variables|Default|GetInventoryHadRoom)
            _
            (else
              (bind _returnvalue (Utilities|GetDataTableRow "/Game/Characters/Player/Inventory/DataStructures/DT_Bullet.DT_Bullet" (Utilities|String|StringToName (Utilities|String|EnumtoString (Utilities|Array|Get(acopy) (Variables|/Game/Characters/Player/BP_Player.BP_Player_C|GetBulletInventory _asbp_player)))))
                (:then
                  (Game|SpawnActorfromClass (.class _returnvalue) (Math|Transform|MakeTransform (+ (Transformation|GetActorLocation Character%20Picking%20Up) (* (Transformation|GetActorForwardVector Character%20Picking%20Up) "60.000000,60.000000,0.000000")) (Transformation|GetActorRotation Character%20Picking%20Up) "1.000000,1.000000,1.000000") "AdjustIfPossibleButAlwaysSpawn" "MultiplyWithRoot" 0 0)
                  (Utilities|Array|SetArrayElem (Variables|/Game/Characters/Player/BP_Player.BP_Player_C|GetBulletInventory _asbp_player) 0 (Variables|Default|GetBulletType) true)))))
          (Actor|DestroyActor))))
    (else
      (goto _label))))

(fn ConstructionScript
  (|CallParentFunction))