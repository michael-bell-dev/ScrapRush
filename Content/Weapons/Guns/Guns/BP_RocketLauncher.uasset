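; BP_RocketLauncher is a rocket launcher gun that adds animation and recoil knockback on top of its parent's logic.
; PlayAnimation plays the fire animation on the skeletal mesh, then launches the owning BP_Player opposite the weapon's right vector.
; The launch overrides horizontal velocity and adds a vertical component damped to a third.
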(event EventBeginPlay
  (|CallParentFunction))

(event EventPlayAnimation
  (bind _returnvalue (Transformation|GetActorRightVector))
  (Components|Animation|PlayAnimation (Variables|Default|GetSkeletalMesh) "/Game/Weapons/MilitaryWeapSilver/Weapons/Animations/Fire_RocketLauncher_W.Fire_RocketLauncher_W" false)
  (bind _asbp_player (Utilities|Casting|CastToBP_Player (Components|GetOwner)))
  (Character|LaunchCharacter _asbp_player (* (Math|Vector|MakeVector (.x _returnvalue) (.y _returnvalue) (/ (.z _returnvalue) 3.0)) -8e+02) true false))

(fn ConstructionScript
  (|CallParentFunction))