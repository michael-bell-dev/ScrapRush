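; Weapon pickup actor that carries a gun's stats and inventory and hands them to the player on interaction, optionally as a purchasable shop item.
; On BeginPlay it derives its price from the product of log-scaled cooldown, velocity, damage and slot count.
; Interact charges shop items if affordable, then calls the player's SpawnWeaponFunction, destroying itself on success; money is deducted before that result is known.
; SetStats overwrites the stats without recomputing the price.
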(event Custom|SetStats
  (params (Cooldown :type Float%20%28double-precision%29) (BulletVelocity :type Float%20%28double-precision%29) (Damage :type Float%20%28double-precision%29) (Lifetime :type Float%20%28double-precision%29) (NumSlots :type Integer) (Inventory :type Array%20of%20E_BulletTypes%20Enums :default "NewEnumerator21"))
  (Variables|Default|SetCooldown Cooldown)
  (Variables|Default|SetBulletVelocity BulletVelocity)
  (Variables|Default|SetDamage Damage)
  (Variables|Default|SetLifetime Lifetime)
  (Variables|Default|SetNumSlots NumSlots)
  (Variables|Default|SetInventory Inventory))

(event Custom|SetValue
  (Variables|Default|SetValue (Math|Float|Truncate (* (Math|Float|Max(Float) (Math|Float|Log (- 1e+01 (Variables|Default|GetCooldown)) 2.0) 1.0) (Math|Float|Max(Float) (Math|Float|Log (Variables|Default|GetBulletVelocity) 2.0) 1.0) (Math|Float|Max(Float) (Math|Float|Log (/ (Variables|Default|GetDamage) 5.0) 2.0) 1.0) (Math|Float|Max(Float) (Math|Float|Log (Math|Conversions|ToFloat(Integer) (Variables|Default|GetNumSlots)) 2.0) 1.0)))))

(event EventBeginPlay
  (|CallParentFunction)
  (CallFunction|SetValue))

(event Collision|EventActorBeginOverlap
  (params (OtherActor :type Actor%20Object%20Reference))
  (|CallParentFunction OtherActor) ; This node is disabled and will not be called.\nDrag off pins to build functionality.
)

(event EventTick
  (params (DeltaSeconds :type Float%20%28single-precision%29))
  (|CallParentFunction DeltaSeconds) ; This node is disabled and will not be called.\nDrag off pins to build functionality.
)

(event EventInteract
  (params (Character%20Picking%20Up :type Actor%20Object%20Reference))
  (bind _value (Variables|Default|GetValue))
  (bind _asbp_player (Utilities|Casting|CastToBP_Player Character%20Picking%20Up))
  (if (Variables|Default|GetShopItem)
    (if (>= (Variables|/Game/Characters/Player/BP_Player.BP_Player_C|GetMoney _asbp_player) _value)
      (Variables|/Game/Characters/Player/BP_Player.BP_Player_C|SetMoney _asbp_player (- (Variables|/Game/Characters/Player/BP_Player.BP_Player_C|GetMoney _asbp_player) _value))
      (bind _output_get (Variables|Default|SetPlayer _asbp_player :!label _label))
      (bind _success (Default|SpawnWeaponFunction _output_get (Variables|Default|GetWeaponToSpawn) (Variables|Default|GetCooldown) (Variables|Default|GetBulletVelocity) (Variables|Default|GetDamage) (Variables|Default|GetLifetime) (Variables|Default|GetNumSlots) (Variables|Default|GetInventory) self (Variables|Default|GetAuto%20Pickup)))
      (if _success
        (Actor|DestroyActor)))
    (else
      (goto _label))))

(fn ConstructionScript
  (|CallParentFunction))