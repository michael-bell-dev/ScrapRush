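; BPC_DamageSystem is a component that manages health, damage, status effects and death for the player and enemies.
; TakeDamage checks immunity, invincibility and blocking, handles lifesteal drops, fires block, response and death dispatchers, and routes Flame and Poison hits to damage-over-time events.
; Fire, poison and gas tick through Delay loops that re-enter TakeDamage as Projectile damage, avoiding re-application.
; It also provides healing, timed immunities with Niagara effects, and temporary Strength weakening.
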(event Custom|Vulnerable
  ;[1 1 1] IFrames
  (Variables|Default|SetIsInvincible false))

(event Custom|Invinsible
  (params (Time :type Float%20%28double-precision%29))
  ;[1 1 1] IFrames
  (Variables|Default|SetIsInvincible true)
  (Utilities|Time|SetTimerbyEvent (delegate Custom|Vulnerable) (Math|Float|Min(Float) (/ Time 2.0) 0.04)))

(event Custom|GrantFireImmunity
  (params (Time :type Float%20%28single-precision%29))
  ;[1 1 1] Disables any further fire damage
  (Utilities|Time|SetTimerbyEvent (delegate Custom|RemoveFireImmunity) Time)
  (Variables|Default|SetImmuneToFire true)
  (Utilities|IsValid (Variables|Default|GetFireImmune)
    (:Is%20Valid
      (Components|DestroyComponent (Variables|Default|GetFireImmune)))
    (:Is%20Not%20Valid
      _))
  (bind _returnvalue (Niagara|SpawnSystemAttached "/Game/M5VFXVOL2/Niagara/Reference/Fire/8_Nflame_pt.8_Nflame_pt" (Variables|/Script/Engine.Actor|GetRootComponent (Components|GetOwner)) "None" "0.000000,0.000000,-5.000000" "0, 0, 0" "KeepRelativeOffset" false))
  (Variables|Default|SetFireImmune _returnvalue))

(event Custom|RemovePoisonImmunity
  (bind _poisonimmune (Variables|Default|GetPoisonImmune))
  ;[1 1 1] Prevents any further poison damage
  (Variables|Default|SetImmuneToPoison false)
  (Utilities|IsValid _poisonimmune
    (:Is%20Valid
      (Components|DestroyComponent _poisonimmune))))

(event Custom|RemoveFireImmunity
  (bind _fireimmune (Variables|Default|GetFireImmune))
  ;[1 1 1] Disables any further fire damage
  (Variables|Default|SetImmuneToFire false)
  (Utilities|IsValid _fireimmune
    (:Is%20Valid
      (Components|DestroyComponent _fireimmune))))

(event Custom|OnFire
  (params (Length :type Integer) (Damage%20Info%20Greater%20Lifesteal :type Boolean) (Damage%20Info%20Attacker :type Actor%20Object%20Reference))
  (bind _returnvalue (Components|GetOwner))
  (bind _rootcomponent (Variables|/Script/Engine.Actor|GetRootComponent _returnvalue))
  ;[1 1 1] Deals repeated fire damage and gives character a fire particle
  (if (not (Variables|Default|GetImmuneToFire))
    (if (Variables|Default|GetEnvironment)
      (if (not (Variables|Default|GetIsDead))
        (Variables|Default|SetFireTick (Math|Float|Ceil (* (Variables|Default|GetMaxHealth) 2.0)))
        (if (not (Variables|Default|GetIsOnFireBool))
          (Transformation|SetWorldScale3D _rootcomponent (/ (Transformation|GetWorldScale _rootcomponent) 0.999999))
          (Variables|Default|SetIsOnFireBool true)
          (Utilities|IsValid (Variables|Default|GetFire)
            (:Is%20Valid
              (Components|Activation|Deactivate (Variables|Default|GetFire))
              (Components|DestroyComponent (Variables|Default|GetFire)))
            (:Is%20Not%20Valid
              _))
          (bind _returnvalue_2 (Niagara|SpawnSystemAttached "/Game/M5VFXVOL2/Niagara/Fire/NFire_12.NFire_12" _rootcomponent "None" "0.000000,0.000000,-5.000000" "0, 0, 0" "KeepRelativeOffset" false))
          (Variables|Default|SetFire _returnvalue_2)
          (Utilities|FlowControl|Delay 0.1 :!label _label)
          (if (or (== (Variables|Default|GetFireTick) 0) (Variables|Default|GetImmuneToFire))
            (Components|Activation|Deactivate (Variables|Default|GetFire))
            (Components|DestroyComponent (Variables|Default|GetFire))
            (Variables|Default|SetIsOnFireBool false)
            (Transformation|SetWorldScale3D _rootcomponent (* (Transformation|GetWorldScale _rootcomponent) 0.999999))
            (else
              (Variables|Default|SetFireTick (- (Variables|Default|GetFireTick) 1))
              (CallFunction|TakeDamage (Utilities|Struct|MakeS_DamageInfo 0.5 "NewEnumerator2" "NewEnumerator1" false false false true 0.0 Damage%20Info%20Greater%20Lifesteal Damage%20Info%20Attacker 0))
              (goto _label)))))
      (else
        (Variables|Default|SetFireTick (+ (Math|Float|Ceil (* (Math|Conversions|ToFloat(Integer) Length) 1.25)) (Variables|Default|GetFireTick)))
        (if (not (Variables|Default|GetIsOnFireBool))
          (Transformation|SetWorldScale3D _rootcomponent (/ (Transformation|GetWorldScale _rootcomponent) 0.999999))
          (Variables|Default|SetIsOnFireBool true)
          (Utilities|IsValid (Variables|Default|GetFire)
            (:Is%20Valid
              (Components|Activation|Deactivate (Variables|Default|GetFire))
              (Components|DestroyComponent (Variables|Default|GetFire)))
            (:Is%20Not%20Valid
              _))
          (Utilities|Casting|CastToBP_EnemyGunhead_Base _returnvalue
            (:then
              (bind _returnvalue_3 (Niagara|SpawnSystemAttached "/Game/M5VFXVOL2/Niagara/Reference/Fireloop/3_Nblowingfire_fwd_pt.3_Nblowingfire_fwd_pt" _rootcomponent "None" "50.000000,0.000000,-100.000000" "0, 0, 0" "KeepRelativeOffset" false))
              (Variables|Default|SetFire _returnvalue_3)
              (goto _label))
            (:CastFailed
              (Utilities|Casting|CastToBP_Player _returnvalue)
              (bind _returnvalue_4 (Niagara|SpawnSystemAttached "/Game/M5VFXVOL2/Niagara/Fire/NFire_00.NFire_00" _rootcomponent "None" "50.000000,0.000000,-100.000000" "0, 0, 0" "KeepRelativeOffset" false))
              (Variables|Default|SetFire _returnvalue_4)
              (goto _label))))))))

(event Custom|Poisoned
  (params (Strength :type Float%20%28double-precision%29) (Damage%20Info%20Greater%20Lifesteal :type Boolean) (Damage%20Info%20Attacker :type Actor%20Object%20Reference))
  (bind _returnvalue (/ Strength 6.0))
  ;[1 1 1] Deals repeated poison damage when poisoned
  (if (not (Variables|Default|GetImmuneToPoison))
    (if (< (Variables|Default|GetPoisonTick) 9)
      (Variables|Default|SetPoisonTick 9)
      (if (Variables|Default|GetIsPoisonedBool)
        (Variables|Default|SetPoisonDamage (+ (Variables|Default|GetPoisonDamage) _returnvalue) :!label _label)
        (else
          (Variables|Default|SetIsPoisonedBool true)
          (Variables|Default|SetPoisonDamage _returnvalue)
          (Utilities|FlowControl|Delay 0.5 :!label _label_2)
          (if (or (== (Variables|Default|GetPoisonTick) 0) (Variables|Default|GetImmuneToPoison))
            (Variables|Default|SetIsPoisonedBool false)
            (else
              (Variables|Default|SetPoisonTick (- (Variables|Default|GetPoisonTick) 1))
              (CallFunction|TakeDamage (Utilities|Struct|MakeS_DamageInfo (Variables|Default|GetPoisonDamage) "NewEnumerator2" "NewEnumerator1" false false false true 0.0 Damage%20Info%20Greater%20Lifesteal Damage%20Info%20Attacker 0))
              (goto _label_2)))))
      (else
        (goto _label)))))

(event Custom|PutOutFire
  ;[1 1 1] Disables fire particle and stops dealing damage
  (if (Variables|Default|GetIsOnFireBool)
    (Variables|Default|SetFireTick 0)
    (Variables|Default|SetIsOnFireBool false)))

(event Custom|Unweaken
  (params (Amount :type Float%20%28double-precision%29) (Duration :type Float%20%28double-precision%29))
  ;[1 1 1] Disable weakness
  (Utilities|FlowControl|Delay Duration)
  (Variables|Default|SetStrength (* (Variables|Default|GetStrength) Amount)))

(event Custom|LethalPoison
  ;[1 1 1] Set poison tick to max if affected by lethal poison
  (Variables|Default|SetPoisonTick 2147483647))

(event Custom|InGas
  (params (InGas :type Boolean) (Strength :type Float%20%28double-precision%29) (Damage%20Info%20Attacker :type Actor%20Object%20Reference))
  ;[1 1 1] Tells DamageSystem character is in toxic gas
  (if InGas
    (Variables|Default|SetPoisonDamage (+ (Variables|Default|GetPoisonDamage) (/ Strength 6.0)))
    (bind _output_get (Variables|Default|SetNumGases (+ (Variables|Default|GetNumGases) 1)))
    (if (== _output_get 1)
      (CallFunction|GasDamage Damage%20Info%20Attacker))
    (else
      (Variables|Default|SetPoisonDamage (- (Variables|Default|GetPoisonDamage) (/ Strength 6.0)))
      (Variables|Default|SetNumGases (+ (Variables|Default|GetNumGases) -1)))))

(event Custom|GrantPoisonImmunity
  (params (Time :type Float%20%28double-precision%29))
  (bind _poison (Variables|Default|GetPoison))
  ;[1 1 1] Prevents any further poison damage
  (Utilities|Time|SetTimerbyEvent (delegate Custom|RemovePoisonImmunity) Time)
  (Variables|Default|SetImmuneToPoison true)
  (Utilities|IsValid _poison
    (:Is%20Valid
      (Components|DestroyComponent _poison))
    (:Is%20Not%20Valid
      _))
  (bind _returnvalue (Niagara|SpawnSystemAttached "/Game/M5VFXVOL2/Niagara/Reference/Fire/8_Nflame_pt.8_Nflame_pt" (Variables|/Script/Engine.Actor|GetRootComponent (Components|GetOwner)) "None" "0.000000,0.000000,-5.000000" "0, 0, 0" "KeepRelativeOffset" false))
  (Variables|Default|SetPoisonImmune _returnvalue))

(event Custom|GasDamage
  (params (DamageInfoAttacker :type Actor%20Object%20Reference))
  ;[1 1 1] Deal damage when character is in toxic gas
  (if (not (Variables|Default|GetImmuneToPoison))
    (CallFunction|TakeDamage (Utilities|Struct|MakeS_DamageInfo (Variables|Default|GetPoisonDamage) "NewEnumerator2" "NewEnumerator1" false false false true 0.0 false DamageInfoAttacker 0))
    (Utilities|FlowControl|Delay 0.2)
    (if (not (== (Variables|Default|GetNumGases) 0))
      (CallFunction|GasDamage DamageInfoAttacker))))

(fn Heal
  (params (Amount :type Float%20%28double-precision%29))
  (if (Variables|Default|GetIsDead)
    (return 0.0)
    (else
      (bind _output_get (Variables|Default|SetHealth (Math|Float|Clamp(Float) (+ Amount (Variables|Default|GetHealth)) 0.0 (Variables|Default|GetMaxHealth))))
      (return _output_get))))

(fn TakeDamage
  (params (DamageInfo :type S%20Damage%20Info%20Structure))
  (bind (_amount _damagetype _damageresponse _shoulddamageinvinsible _canbeblocked _canbeparried _shouldforceinterupt _lifesteal _greaterlifesteal _attacker _droprate) (Utilities|Struct|BreakS_DamageInfo DamageInfo))
  (bind _returnvalue (Components|GetOwner))
  ;[1 1 1] Check id damage should be applied
  (switch Utilities|FlowControl|Switch|SwitchonE_DamageType _damagetype
    (:NewEnumerator1
      (if (not (Variables|Default|GetImmuneToPoison))
        (Utilities|CanbeDamaged _shoulddamageinvinsible _canbeblocked :!label _label
          (:BlockDamage
            (Default|CallOnBlocked _canbeparried)
            (return false))
          (:TakeDamage
            ;[1 1 1] Lifesteal
            (if (> _lifesteal 0.0)
              (if (!= _returnvalue _attacker)
                (bind _asbp_enemy_base (Utilities|Casting|CastToBP_Enemy_Base _returnvalue)
                  (:then
                    (Utilities|Casting|CastToBP_Player _attacker
                      (:then
                        (Default|DropHealth _asbp_enemy_base _lifesteal))
                      (:CastFailed
                        _)))
                  (:CastFailed
                    _))))
            ;[1 1 1] Deal damage
            (if (not (Variables|Default|GetIsDead))
              (bind _output_get (Variables|Default|SetHealth (- (Variables|Default|GetHealth) _amount)))
              (if (<= _output_get 0.0)
                (Variables|Default|SetIsDead true)
                (Variables|Default|SetHealth 0.0)
                ;[1 1 1] Lesser Lifesteal
                (bind _asbp_player (Utilities|Casting|CastToBP_Player (Game|Player|GetPlayerPawn 0))
                  (:then
                    _)
                  (:CastFailed
                    _))
                (bind _asbp_enemy_base_2 (Utilities|Casting|CastToBP_Enemy_Base (Components|GetOwner))
                  (:then
                    (Default|IncreaseDroprate _asbp_enemy_base_2 _droprate)
                    (Default|AddKill _asbp_player)
                    (if _greaterlifesteal
                      (Variables|/Game/Characters/Enemies/BP_Enemy_Base.BP_Enemy_Base_C|SetDropHeart _asbp_enemy_base_2 true)))
                  (:CastFailed
                    _))
                (Default|CallOnDeath)
                ;[1 1 1] Various damage type functions
                (switch Utilities|FlowControl|Switch|SwitchonE_DamageType _damagetype :!label _label_2
                  (:NewEnumerator0
                    (return false))
                  (:NewEnumerator1
                    (CallFunction|Poisoned _amount _greaterlifesteal _attacker))
                  (:NewEnumerator2
                    _)
                  (:NewEnumerator3
                    (CallFunction|OnFire (Math|Float|Ceil _amount) _greaterlifesteal _attacker))
                  (:NewEnumerator4
                    _))
                (return true)
                (elif (or (Variables|Default|GetIsInterruptable) _shouldforceinterupt)
                  (Default|CallOnDamageResponse _damageresponse)
                  (goto _label_2)))))
          (:NoDamage
            (return false)))))
    (:NewEnumerator2
      (goto _label))
    (:NewEnumerator3
      (if (not (Variables|Default|GetImmuneToFire))
        (goto _label)))
    (:NewEnumerator4
      (if (not (Variables|Default|GetImmuneToElectric))
        (goto _label)))))

(fn Invulnerability
  (params (Time :type Float%20%28double-precision%29))
  (CallFunction|Invinsible Time))

(fn IsonFire
  (return (Variables|Default|GetIsOnFireBool)))

(fn Weaken
  (params (Amount :type Float%20%28double-precision%29) (Duration :type Float%20%28double-precision%29))
  (Variables|Default|SetStrength (/ (Variables|Default|GetStrength) Amount))
  (CallFunction|Unweaken Amount Duration))