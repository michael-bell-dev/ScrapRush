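; Enemy Blueprint in the Gunheads folder that fires its weapon constantly at the AI controller's attack target.
; Each Tick, while it is alive and the controller is valid, it checks that the target is not dead, then calls Shoot on the Weapon.
; GetIdealRange functions supply fixed attack and defend radii, with zero attack radius and a short defend radius.
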(event EventBeginPlay
  (|CallParentFunction) ; This node is disabled and will not be called.\nDrag off pins to build functionality.
)

(event Collision|EventActorBeginOverlap
  (params (OtherActor :type Actor%20Object%20Reference)))

(event EventTick
  (params (DeltaSeconds :type Float%20%28single-precision%29))
  (bind _aic_enemy_base (Variables|Default|GetAIC%20Enemy%20Base))
  ;[1 1 1] Constantly attack
  (bind _isdead (CallFunction|IsDead))
  (if (not _isdead)
    (Utilities|IsValid _aic_enemy_base
      (:Is%20Valid
        (bind _isdead_2 (Class|BPIDamagable|IsDead(Message) (Variables|/Game/Characters/Enemies/AI/AIC_Enemy_Base.AIC_Enemy_Base_C|GetAttack%20Target _aic_enemy_base)))
        (if (not _isdead_2)
          (Default|Shoot (Variables|Default|GetWeapon) 0 (Variables|/Game/Characters/Enemies/AI/AIC_Enemy_Base.AIC_Enemy_Base_C|GetAttack%20Target (Variables|Default|GetAIC%20Enemy%20Base))))))))

(fn ConstructionScript
  (|CallParentFunction))

(fn GetIdealRange
  (return 0.0 1e+02))

(fn GetIdealRange1
  (return 0.0 1e+02))

(fn GetIdealRange2
  (return 0.0 1e+02))