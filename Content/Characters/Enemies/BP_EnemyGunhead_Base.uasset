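; Base Blueprint for gunhead enemies, which have their head bone hidden and a weapon attached at the neck in its place.
; ProvideWeapon spawns and configures the weapon, adjusts its transform by type, and optionally starts hostile against the player.
; Attack fires at the AI controller's target with a montage.
; Death rolls ammo and health drops, ragdolls the body, stops AI logic, and destroys both actors after a delay.
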(event Custom|Destroy%20Actors
  ;[1 1 1] Delete Enemy
  (Actor|DestroyActor (Variables|Default|GetWeapon))
  (Actor|DestroyActor))

(event Custom|ProvideWeapon
  ;[1 1 1] Attach weapon to head
  (Components|SkinnedMesh|HideBonebyName (Variables|Character|GetMesh) "Head" "PBO_None")
  (bind _returnvalue (Game|SpawnActorfromClass (Variables|Default|GetWeaponType) (Math|Transform|MakeTransform "0, 0, 0" "0, 0, 0" "1.000000,1.000000,0.000000") "Undefined" "MultiplyWithRoot" self 0))
  (bind _output_get (Variables|Default|SetWeapon _returnvalue))
  (Transformation|AttachComponentToComponent _output_get (Variables|Character|GetMesh) "neck_02" "SnapToTarget" "SnapToTarget" "SnapToTarget" true)
  ;[1 1 1] Set weapon stats
  (Default|SetStats _output_get (Variables|Default|GetCooldown) (Variables|Default|GetBullet%20Velocity) (Variables|Default|GetDamage) (Variables|Default|GetLifetime) (Variables|Default|GetNum%20Slots) (Variables|Default|GetInventory))
  ;[1 1 1] Position each weapon type correctly
  (switch Utilities|FlowControl|Switch|SwitchonE_WeaponName (Variables|/Game/Weapons/Guns/Guns/BP_WeaponBase.BP_WeaponBase_C|GetWeaponName (Variables|Default|GetWeapon))
    (:NewEnumerator0
      (Transformation|SetActorRelativeLocation (Variables|Default|GetWeapon) "-3.000000,1.000000,0.000000")
      (Transformation|SetActorRelativeScale3D (Variables|Default|GetWeapon) "2.000000,2.000000,2.000000"))
    (:NewEnumerator2
      (Transformation|SetActorRelativeLocation (Variables|Default|GetWeapon) "0.000000,-1.000000,0.000000")
      (Transformation|SetActorRelativeScale3D (Variables|Default|GetWeapon) "1.500000,1.500000,1.500000"))
    (:NewEnumerator8
      (Transformation|SetActorRelativeLocation (Variables|Default|GetWeapon) "0.000000,-1.000000,0.000000")
      (Transformation|SetActorRelativeScale3D (Variables|Default|GetWeapon) "1.000000,1.000000,1.000000"))
    (:NewEnumerator1
      (Transformation|SetActorRelativeLocation (Variables|Default|GetWeapon) "0.000000,-1.000000,0.000000")
      (Transformation|SetActorRelativeScale3D (Variables|Default|GetWeapon) "1.000000,1.000000,1.000000"))
    (:NewEnumerator3
      (Transformation|SetActorRelativeLocation (Variables|Default|GetWeapon) "0.000000,-1.000000,0.000000")
      (Transformation|SetActorRelativeScale3D (Variables|Default|GetWeapon) "1.000000,1.000000,1.000000"))
    (:NewEnumerator9
      (Transformation|SetActorRelativeLocation (Variables|Default|GetWeapon))
      (Transformation|SetActorRelativeScale3D (Variables|Default|GetWeapon) "1.000000,1.000000,1.000000"))
    (:NewEnumerator5
      (Transformation|SetActorRelativeLocation (Variables|Default|GetWeapon) "-10.000000,2.000000,0.000000")
      (Transformation|SetActorRelativeScale3D (Variables|Default|GetWeapon) "2.000000,2.000000,2.000000")))
  (Transformation|SetActorRelativeRotation (Variables|Default|GetWeapon) "-90.000000,90.000000,-110.000000")
  ;[1 1 1] Start hostile
  (if (Variables|Default|GetStart%20Hostile)
    (Utilities|FlowControl|Delay 0.5)
    (Default|SetStateasAttacking (Variables|Default|GetAIC%20Enemy%20Base) (Game|Player|GetPlayerPawn 0) false)))

(event EventBeginPlay
  (|CallParentFunction))

(event EventDeath
  (bind _mesh (Variables|Character|GetMesh))
  (bind _aic_enemy_base (Variables|Default|GetAIC%20Enemy%20Base))
  ;[1 1 1] Drop Item When Killed
  (if (> (Math|Random|RandomFloat) (Variables|Default|GetDroprate))
    _
    (else
      (bind _asbp_baserandom_pickup_spawner (Utilities|Casting|CastToBP_BASERandomPickupSpawner (Variables|/Script/Engine.ChildActorComponent|GetChildActor (Variables|Default|GetBulletDrop))))
      (Default|SpawnPickup _asbp_baserandom_pickup_spawner)))
  (CallFunction|DropHealth 0.2)
  ;[1 1 1] Ragdoll
  (CallFunction|DropHealth 0.2)
  (Physics|SetSimulatePhysics _mesh true)
  (Collision|SetCollisionEnabled _mesh "QueryAndPhysics")
  (Collision|SetCollisionEnabled (Variables|Default|GetCapsuleComponent) "NoCollision")
  ;[1 1 1] Kill Enemy
  (AI|Logic|StopLogic (Variables|/Script/AIModule.AIController|GetBrainComponent _aic_enemy_base) "")
  (Default|SetStateasDead _aic_enemy_base)
  (Components|DestroyComponent (Variables|Default|GetHealthBar))
  ;[1 1 1] Delete Enemy
  (Utilities|Time|SetTimerbyEvent (delegate Custom|Destroy%20Actors) 5.0))

(event EventDropHealth
  (params (Chance :type Float%20%28double-precision%29))
  (bind _capsulecomponent (Variables|Default|GetCapsuleComponent))
  (if (or (Variables|Default|GetDropHeart) (< (Math|Random|RandomFloat) Chance))
    (Game|SpawnActorfromClass "/Game/Characters/DamageSystem/Health.Health_C" (Math|Transform|MakeTransform (Transformation|GetWorldLocation _capsulecomponent) (Transformation|GetWorldRotation _capsulecomponent) "0.500000,0.500000,0.500000") "AlwaysSpawn" "MultiplyWithRoot" 0 0)))

(event EventAttack
  ;[1 1 1] Attack Function
  (bind _fired (Default|Shoot (Variables|Default|GetWeapon) 0 (Variables|/Game/Characters/Enemies/AI/AIC_Enemy_Base.AIC_Enemy_Base_C|GetAttack%20Target (Variables|Default|GetAIC%20Enemy%20Base))))
  (if _fired
    (Animation|Montage|PlayMontage (Variables|Character|GetMesh) "/Game/Characters/Mannequins/Animations/Manny/AttackRangedMontage.AttackRangedMontage"
      (:OnCompleted
        _)
      (:OnInterrupted
        _))
    (Default|CallOnAttackEnd)))

(fn ConstructionScript
  (|CallParentFunction))

(fn GetIdealRange
  (return 1e+03 1.5e+03))

(fn GetIdealRange0
  (return 0.0 1e+02))