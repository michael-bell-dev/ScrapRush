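; Flammable world object that catches fire from burning actors it hits and spreads it to objects, enemies and the player.
; BPC_DamageSystem handles its randomized health and burn state behind damage interface functions, with health getters and Heal stubbed.
; Cube hits record touching actors, never removed, and pass on fire damage using random chances and delays.
; On death, a burning object damages those actors, harder if characters aren't alight, then destroys itself.
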(event OnDeath(BPC_DamageSystem)
  (bind _onfire (CallFunction|GetonFire))
  (if _onfire
    (for _array_element (Variables|Default|GetTouchingActors)
      (Utilities|IsValid _array_element
        (:Is%20Valid
          (bind _asbp_flamable_object (Utilities|Casting|CastToBP_FlamableObject _array_element)
            (:then
              (if (not (== (Math|Random|RandomInteger 5) 0))
                (Class|BPIDamagable|TakeDamage(Message) (Variables|BP_FlamableObject_C|GetBPC_DamageSystem _asbp_flamable_object) (Utilities|Struct|MakeS_DamageInfo 0.5 "NewEnumerator3" "NewEnumerator2" false false false true 0.0 false 0 0))))
            (:CastFailed
              (bind _asbp_enemy_base (Utilities|Casting|CastToBP_Enemy_Base (stale OnComponentHit(Cube) _array_element))
                (:then
                  (bind _onfire_2 (Default|IsonFire (Variables|/Game/Characters/Enemies/BP_Enemy_Base.BP_Enemy_Base_C|GetBPC_DamageSystem _asbp_enemy_base)))
                  (if _onfire_2
                    (Class|BPIDamagable|TakeDamage(Message) (Variables|/Game/Characters/Enemies/BP_Enemy_Base.BP_Enemy_Base_C|GetBPC_DamageSystem _asbp_enemy_base) (Utilities|Struct|MakeS_DamageInfo 2.0 "NewEnumerator3" "NewEnumerator2" false false false true 0.0 false 0 0))
                    (else
                      (Class|BPIDamagable|TakeDamage(Message) (Variables|/Game/Characters/Enemies/BP_Enemy_Base.BP_Enemy_Base_C|GetBPC_DamageSystem _asbp_enemy_base) (Utilities|Struct|MakeS_DamageInfo 15.0 "NewEnumerator3" "NewEnumerator2" false false false true 0.0 false 0 0)))))
                (:CastFailed
                  (bind _asbp_player (Utilities|Casting|CastToBP_Player (stale OnComponentHit(Cube) _array_element)))
                  (bind _onfire_3 (Default|IsonFire (Variables|/Game/Characters/Player/BP_Player.BP_Player_C|GetBPC_DamageSystem _asbp_player)))
                  (if _onfire_3
                    (Class|BPIDamagable|TakeDamage(Message) (Variables|/Game/Characters/Player/BP_Player.BP_Player_C|GetBPC_DamageSystem _asbp_player) (Utilities|Struct|MakeS_DamageInfo 1.0 "NewEnumerator3" "NewEnumerator2" false false false true 0.0 false 0 0))
                    (else
                      (Class|BPIDamagable|TakeDamage(Message) (Variables|/Game/Characters/Player/BP_Player.BP_Player_C|GetBPC_DamageSystem _asbp_player) (Utilities|Struct|MakeS_DamageInfo 5.0 "NewEnumerator3" "NewEnumerator2" false false false true 0.0 false 0 0))))))))))))
  (Actor|DestroyActor))

(event OnComponentHit(Cube)
  (params (HitComponent :type Primitive%20Component%20Object%20Reference) (OtherActor :type Actor%20Object%20Reference) (OtherComp :type Primitive%20Component%20Object%20Reference) (NormalImpulse :type Vector :default "0, 0, 0") (Hit :type Hit%20Result%20Structure%20%28by%20ref%29))
  (bind _touchingactors (Variables|Default|GetTouchingActors))
  (bind _asbpi_damagable (Utilities|Casting|CastToBPI_Damagable OtherActor))
  (if (Utilities|Array|ContainsItem _touchingactors OtherActor)
    _
    (else
      (Utilities|Array|Add _touchingactors OtherActor)))
  (bind _onfire (Default|GetonFire _asbpi_damagable))
  (if _onfire
    (Utilities|Casting|CastToBP_FlamableObject OtherActor
      (:then
        (Utilities|FlowControl|Delay (+ (* (Math|Random|RandomFloat) 2.0) 1.0))
        (Utilities|IsValid (Utilities|ToObject(Interface) _asbpi_damagable)
          (:Is%20Valid
            (bind _onfire_2 (Default|GetonFire _asbpi_damagable))
            (if _onfire_2
              (if (not (== (Math|Random|RandomInteger 5) 0)) :!label _label
                (CallFunction|TakeDamage (Utilities|Struct|MakeS_DamageInfo 0.1 "NewEnumerator3" "NewEnumerator2" false false false true 0.0 false 0 0))
                (for _array_element (Variables|Default|GetTouchingActors)
                  (Utilities|IsValid _array_element
                    (:Is%20Valid
                      (bind _asbp_flamable_object (Utilities|Casting|CastToBP_FlamableObject _array_element)
                        (:then
                          (Utilities|FlowControl|Delay (+ (* (Math|Random|RandomFloat) 2.0) 1.0))
                          (Utilities|IsValid _asbp_flamable_object
                            (:Is%20Valid
                              (bind _onfire_3 (CallFunction|GetonFire))
                              (if _onfire_3
                                (Class|BPIDamagable|TakeDamage(Message) (Variables|BP_FlamableObject_C|GetBPC_DamageSystem _asbp_flamable_object) (Utilities|Struct|MakeS_DamageInfo 0.5 "NewEnumerator3" "NewEnumerator2" false false false true 0.0 false 0 0))))))
                        (:CastFailed
                          (bind _asbp_enemy_base (Utilities|Casting|CastToBP_Enemy_Base _array_element)
                            (:then
                              (bind _onfire_4 (Default|IsonFire (Variables|/Game/Characters/Enemies/BP_Enemy_Base.BP_Enemy_Base_C|GetBPC_DamageSystem _asbp_enemy_base)))
                              (if _onfire_4
                                (Class|BPIDamagable|TakeDamage(Message) (Variables|/Game/Characters/Enemies/BP_Enemy_Base.BP_Enemy_Base_C|GetBPC_DamageSystem _asbp_enemy_base) (Utilities|Struct|MakeS_DamageInfo 2.0 "NewEnumerator3" "NewEnumerator2" false false false true 0.0 false 0 0))
                                (else
                                  (Class|BPIDamagable|TakeDamage(Message) (Variables|/Game/Characters/Enemies/BP_Enemy_Base.BP_Enemy_Base_C|GetBPC_DamageSystem _asbp_enemy_base) (Utilities|Struct|MakeS_DamageInfo 15.0 "NewEnumerator3" "NewEnumerator2" false false false true 0.0 false 0 0)))))
                            (:CastFailed
                              (bind _asbp_player (Utilities|Casting|CastToBP_Player _array_element))
                              (bind _onfire_5 (Default|IsonFire (Variables|/Game/Characters/Player/BP_Player.BP_Player_C|GetBPC_DamageSystem _asbp_player)))
                              (if _onfire_5
                                (Class|BPIDamagable|TakeDamage(Message) (Variables|/Game/Characters/Player/BP_Player.BP_Player_C|GetBPC_DamageSystem _asbp_player) (Utilities|Struct|MakeS_DamageInfo 1.0 "NewEnumerator3" "NewEnumerator2" false false false true 0.0 false 0 0))
                                (else
                                  (Class|BPIDamagable|TakeDamage(Message) (Variables|/Game/Characters/Player/BP_Player.BP_Player_C|GetBPC_DamageSystem _asbp_player) (Utilities|Struct|MakeS_DamageInfo 5.0 "NewEnumerator3" "NewEnumerator2" false false false true 0.0 false 0 0))))))))))))))
          (:Is%20Not%20Valid
            (goto _label))))
      (:CastFailed
        (goto _label)))))

(event EventBeginPlay
  (bind _bpc_damagesystem (Variables|Default|GetBPC_DamageSystem))
  (bind _output_get (Variables|Default|SetNewHealth (+ (Variables|Default|GetNewHealth) (- (* (Math|Random|RandomFloat) 5e+01) 25.0))))
  (Variables|/Game/Characters/DamageSystem/BPC_DamageSystem.BPC_DamageSystem_C|SetMaxHealth _bpc_damagesystem _output_get)
  (Variables|/Game/Characters/DamageSystem/BPC_DamageSystem.BPC_DamageSystem_C|SetHealth _bpc_damagesystem _output_get))

(event EventPutOutFire
  (Default|PutOutFire (Variables|Default|GetBPC_DamageSystem)))

(fn ConstructionScript)

(fn GetCurrentHealth
  (return 0.0))

(fn GetMaxHealth
  (return 0.0))

(fn GetonFire
  (bind _onfire (Default|IsonFire (Variables|Default|GetBPC_DamageSystem)))
  (return _onfire))

(fn Heal
  (params (Amount :type Float%20%28double-precision%29))
  (return 0.0))

(fn IsDead
  (bind _isdead (Class|BPIDamagable|IsDead(Message) (Variables|Default|GetBPC_DamageSystem)))
  (return _isdead))

(fn TakeDamage
  (params (DamageInfo :type S%20Damage%20Info%20Structure))
  (Default|TakeDamage (Variables|Default|GetBPC_DamageSystem) DamageInfo)
  (return false))