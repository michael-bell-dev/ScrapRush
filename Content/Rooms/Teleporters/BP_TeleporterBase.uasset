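; Base teleporter actor that moves an interacting character to a destination elsewhere in the level.
; On Interact it finds an actor of the TeleportDestination class, places the character slightly above it without sweeping, then notifies the BP_Player cached at BeginPlay.
; SetActive turns on the sphere's overlap events and swaps the mesh to a gold material to show the teleporter is active.
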(event Custom|SetActive
  (Variables|/Script/Engine.PrimitiveComponent|SetbGenerateOverlapEvents (Variables|Default|GetSphere) true)
  (Rendering|Material|SetMaterial (Variables|Default|GetStaticMesh) 0 "/Game/Weapons/Bullets/BulletMaterials/Gold.Gold"))

(event EventBeginPlay
  (bind _asbp_player (Utilities|Casting|CastToBP_Player (Game|Player|GetPlayerPawn 0)))
  (Variables|Default|SetPlayer _asbp_player))

(event Collision|EventActorBeginOverlap
  (params (OtherActor :type Actor%20Object%20Reference)))

(event EventTick
  (params (DeltaSeconds :type Float%20%28single-precision%29)))

(event EventInteract
  (params (Character%20Picking%20Up :type Actor%20Object%20Reference))
  (bind _returnvalue (Actor|GetActorOfClass (Variables|Default|GetTeleportDestination)))
  (Transformation|SetActorLocation Character%20Picking%20Up (+ (Transformation|GetActorLocation _returnvalue) "0.000000,0.000000,100.000000") false true)
  (Default|PlayerTeleported (Variables|Default|GetPlayer)))

(fn ConstructionScript
  (|CallParentFunction))